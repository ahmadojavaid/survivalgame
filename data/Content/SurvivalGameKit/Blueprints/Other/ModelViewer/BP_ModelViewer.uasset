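; Model viewer actor that shows a copy of the character's equipment and renders it to two render textures through scene capture components.
; UpdateCharacterEquipment swaps the head, chest, legs, feet or backpack mesh from the equipped item's details; these parts follow the base skeletal mesh via master pose.
; In performance mode, per-frame capture is switched off and both captures render once after each equipment change.
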(event `Update Character Equipment`
  (params (`Equipment Slot` :type "/Game/SurvivalGameKit/Blueprints/Other/S_EquipmentSlot Structure"))
  (bind (_slottype _equipteditem) (break `/Game/SurvivalGameKit/Blueprints/Other/S_EquipmentSlot` `Equipment Slot`))
  ;[1 1 1] Update model viewer character
  (`SkinnedMeshComponent.SetSkinnedAssetAndUpdate` (select `/Game/SurvivalGameKit/Blueprints/Other/Enums/E_EquipmentCategorys` _slottype :`NewEnumerator1` (`self.Backpack`) :`NewEnumerator2` (`self.Feet`) :`NewEnumerator3` (`self.Head`) :`NewEnumerator4` (`self.Chest`) :`NewEnumerator5` (`self.Legs`) :!type "SkinnedMeshComponent Object Reference") (`.EquippedMesh_92_18E57AC5491B8222B0CEE6AC4E6AC9A0` (break `/Game/SurvivalGameKit/Blueprints/Other/S_ItemDetails` (`.Item Details Out` (`/Game/SurvivalGameKit/Blueprints/Other/Libraries/BP_InventoryFunctions.Item Details` _equipteditem)))) true)
  ;[1 1 1] Is in preformance mode
  (if (`self.Preformance Mode`)
    ;[1 1 1] Capture character once
    (`SceneCaptureComponent2D.CaptureScene` (`self.CaptureComponent`))
    (`SceneCaptureComponent2D.CaptureScene` (`self.SceneCaptureComponent2D`))))

(event `self.ReceiveBeginPlay`
  ;[1 1 1] Is in preformance mode
  (if (`self.Preformance Mode`) :!label _label
    ;[1 1 1] Dont capture every frame
    (set `SceneCaptureComponent.bCaptureEveryFrame` false (`self.CaptureComponent`))
    (set `SceneCaptureComponent.bCaptureEveryFrame` false (`self.SceneCaptureComponent2D`))))

(event `On Spawned`
  ;[1 1 1] Set render textures
  (set `SceneCaptureComponent2D.TextureTarget` "/Game/SurvivalGameKit/Blueprints/Other/ModelViewer/RT_ModelViewerOutput.RT_ModelViewerOutput" (`self.CaptureComponent`))
  (set `SceneCaptureComponent2D.TextureTarget` "/Game/SurvivalGameKit/Blueprints/Other/ModelViewer/RT_ModelViewerOutput2.RT_ModelViewerOutput2" (`self.SceneCaptureComponent2D`))
  (goto _label))

(fn `UserConstructionScript`
  (bind _skeletalmesh (`self.SkeletalMesh`))
  (`SkinnedMeshComponent.SetLeaderPoseComponent` (`self.Head`) _skeletalmesh)
  (`SkinnedMeshComponent.SetLeaderPoseComponent` (`self.Chest`) _skeletalmesh)
  (`SkinnedMeshComponent.SetLeaderPoseComponent` (`self.Legs`) _skeletalmesh)
  (`SkinnedMeshComponent.SetLeaderPoseComponent` (`self.Feet`) _skeletalmesh)
  (`SkinnedMeshComponent.SetLeaderPoseComponent` (`self.Backpack`) _skeletalmesh))