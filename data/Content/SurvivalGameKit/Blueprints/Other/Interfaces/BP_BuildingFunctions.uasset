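; Shared building helper functions for the survival game kit, covering placement math, build part data and repair pricing.
; VectorTransform offsets a transform's location along its own forward, right and up axes.
; BuildPartInfoHandle resolves a row handle's name in the BuildPartList data table and reports whether it was found.
; BuildingRepairCost converts health into whole tenths of maximum and returns the missing tenths as the cost, zero at ten.
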(fn `Build Part Info Handle`
  (params (`Build Part Handle` :type "DataTableRowHandle Structure"))
  (returns (`Return Value` :type Boolean) (`Build Part Info` :type "/Game/SurvivalGameKit/Blueprints/Other/S_BuildPartInfo Structure"))
  (bind _returnvalue (`|GetDataTableRow` "/Game/SurvivalGameKit/Blueprints/BuildParts/BuildPartList.BuildPartList" (`.RowName` (break `DataTableRowHandle` `Build Part Handle`)))
    (:`then`
      (return true _returnvalue))
    (:`RowNotFound`
      (return false _returnvalue))))

(fn `Building Repair Cost`
  (params (Building :type "/Game/SurvivalGameKit/Blueprints/BuildParts/BP_MasterBuildPart Object Reference"))
  (returns (`Repair Item Count` :type Integer))
  (locals (`Start Percent` :type Integer))
  (bind (_remainder _returnvalue) (`KismetMathLibrary.FMod` (`KismetMathLibrary.Conv_IntToDouble` (`/Game/SurvivalGameKit/Blueprints/BuildParts/BP_MasterBuildPart.Current Health` Building)) (`KismetMathLibrary.Conv_IntToDouble` (/ (`/Game/SurvivalGameKit/Blueprints/BuildParts/BP_MasterBuildPart.Max Health` Building) 10))))
  (set `local.Start Percent` _returnvalue)
  (if (== _returnvalue 10)
    (return 0)
    (else
      (return (- 10 (`local.Start Percent`))))))

(fn `Vector Transform`
  (params (`Input Transform` :type "Transform Structure") (`Input Forward` :type "Float (double-precision)") (`Input Right` :type "Float (double-precision)") (`Input Up` :type "Float (double-precision)"))
  (returns (`Output Vector` :type "Vector Structure"))
  (bind _rotation (.rotation `Input Transform`))
  ;[1 1 1] We use this to move in the x, y, z axis of the transform
  (return (+ (.location `Input Transform`) (* (`KismetMathLibrary.GetForwardVector` _rotation) `Input Forward`) (* (`KismetMathLibrary.GetRightVector` _rotation) `Input Right`) (* (`KismetMathLibrary.GetUpVector` _rotation) `Input Up`))))