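; Blueprint interface for the Survival Game Kit that declares shared calls for interaction, held items, inventory and damage.
; Interaction functions cover prompt name, action text, input brush, timed interactions with cancel and done callbacks, targeting and animation toggles.
; Item functions forward key and mouse input and handle reloading, unequipping, attachments and their stats, and building options.
; Other functions handle inventory slot changes, hitbox damage and repeating bleed damage.
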(fn `Add Attachment`
  (params (Attachment :type "/Game/SurvivalGameKit/Blueprints/Attachments/BP_MasterAttachment Class Reference")))

(fn `Add Attachment Stats`
  (params (Attachment :type "/Game/SurvivalGameKit/Blueprints/Attachments/BP_MasterAttachment Object Reference")))

(fn `Add Inventory Slots`
  (params (`Index Array` :type "Array of Integer")))

(fn `B Input Action`
  (params (`Key Down` :type Boolean)))

(fn `Bleed Damage`
  (params (`Bleed Repeat Time` :type "Float (double-precision)") (`Bleed Length` :type "Float (double-precision)") (`Bleed Damage` :type Integer)))

(fn `Building Options`
  (params (`Player Inventory Component` :type "/Game/SurvivalGameKit/Blueprints/Components/BP_PlayerInventoryComponent Object Reference")))

(fn `Close Interact Animation`)

(fn `Convert Item Check`)

(fn `Damage`
  (params (Hitbox :type "/Game/SurvivalGameKit/Blueprints/Other/Enums/E_HitboxType Enum" :default "NewEnumerator0") (Damage :type Integer)))

(fn `F Input Action`
  (params (`Key Down` :type Boolean)))

(fn `Interact`
  (params (`Player Component` :type "/Game/SurvivalGameKit/Blueprints/Components/BP_PlayerInventoryComponent Object Reference")))

(fn `Interact Action`
  (returns (`Interact Action Text` :type Text))
  (return ""))

(fn `Interact Cancelled`)

(fn `Interact Done`)

(fn `Interact Input Brush`
  (returns (Brush :type "SlateBrush Structure"))
  (return))

(fn `Interact Name`
  (returns (`Instace Text` :type Text))
  (return ""))

(fn `Interact Time`
  (returns (`Interact Time` :type Boolean) (Time :type "Float (double-precision)"))
  (return false 0.0))

(fn `Interacting Action Text`
  (returns (Text :type Text))
  (return ""))

(fn `Is Interactable`
  (returns (Interactable :type Boolean))
  (return false))

(fn `Left Mouse Input Action`
  (params (`Key Down` :type Boolean)))

(fn `Move Inventory Item`
  (params (`Start Item` :type "/Game/SurvivalGameKit/Blueprints/Other/S_ItemInventory Structure") (`End Item` :type "/Game/SurvivalGameKit/Blueprints/Other/S_ItemInventory Structure")))

(fn `Not Target`)

(fn `On Unequip`)

(fn `Open Interact Animation`)

(fn `Q Input Action`
  (params (`Key Down` :type Boolean)))

(fn `R Input Action`
  (params (`Key Down` :type Boolean)))

(fn `Reload`)

(fn `Remove All Attachments`)

(fn `Remove Attachment`
  (params (Attachment :type "/Game/SurvivalGameKit/Blueprints/Other/Enums/E_AttachmentType Enum" :default "NewEnumerator0") (`Remove Class` :type Boolean)))

(fn `Remove Attachment Stats`
  (params (Attachment :type "/Game/SurvivalGameKit/Blueprints/Attachments/BP_MasterAttachment Object Reference") (`Remove Class` :type Boolean)))

(fn `Remove Inventory Slot`)

(fn `Reset Holdable`)

(fn `Switch Off Interact Animation`)

(fn `Switch On Interact Animation`)

(fn `Target`)

(fn `Toggle Component`)