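; BP_WoodChest is a useable wooden chest in the survival game kit that reacts to player targeting and to open and close interactions.
; Client-side target events toggle custom depth rendering on its mesh while a player aims at it.
; Server-side interaction events show the open and closed states by swapping the static mesh rather than playing an animation.
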(event `/Game/SurvivalGameKit/Blueprints/Other/Interfaces/BP_SurvivalInventoryInterface.Target`
  ;[0 0.5089 1] Client events
  ;;[1 1 1] Player target
  (`PrimitiveComponent.SetRenderCustomDepth` (`self.Mesh`) true))

(event `/Game/SurvivalGameKit/Blueprints/Other/Interfaces/BP_SurvivalInventoryInterface.Open Interact Animation`
  ;[0 1 0.09084] Server events
  ;;[1 1 1] Set open static mesh
  (`StaticMeshComponent.SetStaticMesh` (`self.Mesh`) "/Game/SurvivalGameKit/Meshes/StaticMeshes/SM_Fire_Treasure002.SM_Fire_Treasure002"))

(event `/Game/SurvivalGameKit/Blueprints/Other/Interfaces/BP_SurvivalInventoryInterface.Not Target`
  ;[0 0.5089 1] Client events
  ;;[1 1 1] Not a player target
  (`PrimitiveComponent.SetRenderCustomDepth` (`self.Mesh`) false))

(event `/Game/SurvivalGameKit/Blueprints/Other/Interfaces/BP_SurvivalInventoryInterface.Close Interact Animation`
  ;[0 1 0.09084] Server events
  ;;[1 1 1] Set closed static mesh
  (`StaticMeshComponent.SetStaticMesh` (`self.Mesh`) "/Game/SurvivalGameKit/Meshes/StaticMeshes/SM_Fire_Treasure003.SM_Fire_Treasure003"))

(fn `UserConstructionScript`)