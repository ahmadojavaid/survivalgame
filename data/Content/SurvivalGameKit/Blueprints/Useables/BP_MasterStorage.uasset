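; Base interactable storage actor for the survival kit, serving as a container the player can use.
; Interaction functions supply the action text, input brush, storage name and optional hold time, while the server-side Interact event hands the player component to StorageInventoryComponent.
; The InteractTime query also spawns the timer sound as a side effect, which the client-side done and cancelled events stop.
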(event `/Game/SurvivalGameKit/Blueprints/Other/Interfaces/BP_SurvivalInventoryInterface.Interact Done`
  (bind _interact_sound (`self.Interact Sound`))
  ;[0 0.5089 1] Client events
  ;;[1 1 1] Interaction timer done
  (`/Engine/EditorBlueprintResources/StandardMacros.IsValid` _interact_sound
    (:`Is Valid`
      (`AudioComponent.Stop` _interact_sound))))

(event `/Game/SurvivalGameKit/Blueprints/Other/Interfaces/BP_SurvivalInventoryInterface.Interact Cancelled`
  (bind _interact_sound (`self.Interact Sound`))
  ;[0 0.5089 1] Client events
  ;;[1 1 1] Interact timer cancelled
  (`/Engine/EditorBlueprintResources/StandardMacros.IsValid` _interact_sound
    (:`Is Valid`
      (`AudioComponent.Stop` _interact_sound))))

(event `/Game/SurvivalGameKit/Blueprints/Other/Interfaces/BP_SurvivalInventoryInterface.Interact`
  (params (`Player Component` :type "/Game/SurvivalGameKit/Blueprints/Components/BP_PlayerInventoryComponent Object Reference"))
  ;[0 1 0.09084] Server events
  ;;[1 1 1] Interact event passed to component
  (`/Game/SurvivalGameKit/Blueprints/Other/Interfaces/BP_SurvivalInventoryInterface.Interact` (`self.StorageInventoryComponent`) `Player Component`))

(fn `Interact Action`
  (returns (`Interact Action Text` :type Text))
  (return (`self.Interact Action Text`)))

(fn `Interact Input Brush`
  (returns (Brush :type "SlateBrush Structure"))
  (return (`self.Interact Brush`)))

(fn `Interact Name`
  (returns (`Instace Text` :type Text))
  (return (`KismetTextLibrary.Conv_StringToText` (`/Game/SurvivalGameKit/Blueprints/Components/BP_StorageInventoryComponent.Storage Name` (`self.StorageInventoryComponent`)))))

(fn `Interact Time`
  (returns (`Interact Time` :type Boolean) (Time :type "Float (double-precision)"))
  ;[1 1 1] Interact time
  (if (`self.Use Interact Time`)
    ;;[1 1 1] Is sound set
    (`/Engine/EditorBlueprintResources/StandardMacros.IsValid` (`self.Interact Timer Sound`)
      (:`Is Valid`
        ;;[1 1 1] Play the sound at location
        (bind _returnvalue (`GameplayStatics.SpawnSoundAtLocation` (`self.Interact Timer Sound`) (`self.K2_GetActorLocation`)))
        (set `self.Interact Sound` _returnvalue)
        (return (`self.Use Interact Time`) (`self.Time To Interact`)))
      (:`Is Not Valid`
        (return (`self.Use Interact Time`) (`self.Time To Interact`))))
    (else
      (return false 0.0))))

(fn `Interacting Action Text`
  (returns (Text :type Text))
  (return (`self.Interact Timer Text`)))

(fn `Is Interactable`
  (returns (Interactable :type Boolean))
  (return true))

(fn `UserConstructionScript`)