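; Base world pickup item for the survival kit, interacted with to be picked up through the player component, with optional timed pickup.
; Construction sets static or skeletal mesh from the item's data row.
; On BeginPlay, weapons have the server spawn socketed attachment actors, using range class defaults unless player-dropped; destroying the item removes them.
; Targeting toggles custom depth on meshes and attachments for highlighting.
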(event `/Game/SurvivalGameKit/Blueprints/Other/Interfaces/BP_SurvivalInventoryInterface.Not Target`
  (bind _sight (`self.Sight`))
  (bind _front_grip (`self.Front Grip`))
  (bind _magazine (`self.Magazine`))
  (bind _stock (`self.Stock`))
  (bind _trigger (`self.Trigger`))
  (bind _handguard (`self.Handguard`))
  (bind _underbarrel (`self.Underbarrel`))
  (bind _muzzle (`self.Muzzle`))
  (bind _wrap (`self.Wrap`))
  (`PrimitiveComponent.SetRenderCustomDepth` (`self.Static World Mesh`) false)
  (`PrimitiveComponent.SetRenderCustomDepth` (`self.Skeletal World Mesh`) false)
  (`/Engine/EditorBlueprintResources/StandardMacros.IsValid` _sight
    (:`Is Valid`
      (`PrimitiveComponent.SetRenderCustomDepth` (`/Game/SurvivalGameKit/Blueprints/Attachments/BP_MasterAttachment.Attachment Mesh` _sight) false))
    (:`Is Not Valid`
      _))
  (`/Engine/EditorBlueprintResources/StandardMacros.IsValid` _front_grip
    (:`Is Valid`
      (`PrimitiveComponent.SetRenderCustomDepth` (`/Game/SurvivalGameKit/Blueprints/Attachments/BP_MasterAttachment.Attachment Mesh` _front_grip) false))
    (:`Is Not Valid`
      _))
  (`/Engine/EditorBlueprintResources/StandardMacros.IsValid` _magazine
    (:`Is Valid`
      (`PrimitiveComponent.SetRenderCustomDepth` (`/Game/SurvivalGameKit/Blueprints/Attachments/BP_MasterAttachment.Attachment Mesh` _magazine) false))
    (:`Is Not Valid`
      _))
  (`/Engine/EditorBlueprintResources/StandardMacros.IsValid` _stock
    (:`Is Valid`
      (`PrimitiveComponent.SetRenderCustomDepth` (`/Game/SurvivalGameKit/Blueprints/Attachments/BP_MasterAttachment.Attachment Mesh` _stock) false))
    (:`Is Not Valid`
      _))
  (`/Engine/EditorBlueprintResources/StandardMacros.IsValid` _trigger
    (:`Is Valid`
      (`PrimitiveComponent.SetRenderCustomDepth` (`/Game/SurvivalGameKit/Blueprints/Attachments/BP_MasterAttachment.Attachment Mesh` _trigger) false))
    (:`Is Not Valid`
      _))
  (`/Engine/EditorBlueprintResources/StandardMacros.IsValid` _handguard
    (:`Is Valid`
      (`PrimitiveComponent.SetRenderCustomDepth` (`/Game/SurvivalGameKit/Blueprints/Attachments/BP_MasterAttachment.Attachment Mesh` _handguard) false))
    (:`Is Not Valid`
      _))
  (`/Engine/EditorBlueprintResources/StandardMacros.IsValid` _underbarrel
    (:`Is Valid`
      (`PrimitiveComponent.SetRenderCustomDepth` (`/Game/SurvivalGameKit/Blueprints/Attachments/BP_MasterAttachment.Attachment Mesh` _underbarrel) false))
    (:`Is Not Valid`
      _))
  (`/Engine/EditorBlueprintResources/StandardMacros.IsValid` _muzzle
    (:`Is Valid`
      (`PrimitiveComponent.SetRenderCustomDepth` (`/Game/SurvivalGameKit/Blueprints/Attachments/BP_MasterAttachment.Attachment Mesh` _muzzle) false))
    (:`Is Not Valid`
      _))
  (`/Engine/EditorBlueprintResources/StandardMacros.IsValid` _wrap
    (:`Is Valid`
      (`PrimitiveComponent.SetRenderCustomDepth` (`/Game/SurvivalGameKit/Blueprints/Attachments/BP_MasterAttachment.Attachment Mesh` _wrap) false))))

(event `/Game/SurvivalGameKit/Blueprints/Other/Interfaces/BP_SurvivalInventoryInterface.Target`
  (bind _underbarrel (`self.Underbarrel`))
  (bind _muzzle (`self.Muzzle`))
  (bind _sight (`self.Sight`))
  (bind _front_grip (`self.Front Grip`))
  (bind _magazine (`self.Magazine`))
  (bind _stock (`self.Stock`))
  (bind _wrap (`self.Wrap`))
  (bind _trigger (`self.Trigger`))
  (bind _handguard (`self.Handguard`))
  (`/Engine/EditorBlueprintResources/StandardMacros.IsValid` _sight
    (:`Is Valid`
      (`PrimitiveComponent.SetRenderCustomDepth` (`/Game/SurvivalGameKit/Blueprints/Attachments/BP_MasterAttachment.Attachment Mesh` _sight) true))
    (:`Is Not Valid`
      _))
  (`/Engine/EditorBlueprintResources/StandardMacros.IsValid` _front_grip
    (:`Is Valid`
      (`PrimitiveComponent.SetRenderCustomDepth` (`/Game/SurvivalGameKit/Blueprints/Attachments/BP_MasterAttachment.Attachment Mesh` _front_grip) true))
    (:`Is Not Valid`
      _))
  (`/Engine/EditorBlueprintResources/StandardMacros.IsValid` _magazine
    (:`Is Valid`
      (`PrimitiveComponent.SetRenderCustomDepth` (`/Game/SurvivalGameKit/Blueprints/Attachments/BP_MasterAttachment.Attachment Mesh` _magazine) true))
    (:`Is Not Valid`
      _))
  (`/Engine/EditorBlueprintResources/StandardMacros.IsValid` _stock
    (:`Is Valid`
      (`PrimitiveComponent.SetRenderCustomDepth` (`/Game/SurvivalGameKit/Blueprints/Attachments/BP_MasterAttachment.Attachment Mesh` _stock) true))
    (:`Is Not Valid`
      _))
  (`/Engine/EditorBlueprintResources/StandardMacros.IsValid` _trigger
    (:`Is Valid`
      (`PrimitiveComponent.SetRenderCustomDepth` (`/Game/SurvivalGameKit/Blueprints/Attachments/BP_MasterAttachment.Attachment Mesh` _trigger) true))
    (:`Is Not Valid`
      _))
  (`/Engine/EditorBlueprintResources/StandardMacros.IsValid` _handguard
    (:`Is Valid`
      (`PrimitiveComponent.SetRenderCustomDepth` (`/Game/SurvivalGameKit/Blueprints/Attachments/BP_MasterAttachment.Attachment Mesh` _handguard) true))
    (:`Is Not Valid`
      _))
  (`/Engine/EditorBlueprintResources/StandardMacros.IsValid` _underbarrel
    (:`Is Valid`
      (`PrimitiveComponent.SetRenderCustomDepth` (`/Game/SurvivalGameKit/Blueprints/Attachments/BP_MasterAttachment.Attachment Mesh` _underbarrel) true))
    (:`Is Not Valid`
      _))
  (`/Engine/EditorBlueprintResources/StandardMacros.IsValid` _muzzle
    (:`Is Valid`
      (`PrimitiveComponent.SetRenderCustomDepth` (`/Game/SurvivalGameKit/Blueprints/Attachments/BP_MasterAttachment.Attachment Mesh` _muzzle) true))
    (:`Is Not Valid`
      _))
  (`/Engine/EditorBlueprintResources/StandardMacros.IsValid` _wrap
    (:`Is Valid`
      (`PrimitiveComponent.SetRenderCustomDepth` (`/Game/SurvivalGameKit/Blueprints/Attachments/BP_MasterAttachment.Attachment Mesh` _wrap) true))
    (:`Is Not Valid`
      _))
  (`PrimitiveComponent.SetRenderCustomDepth` (`self.Static World Mesh`) true)
  (`PrimitiveComponent.SetRenderCustomDepth` (`self.Skeletal World Mesh`) true))

(event `/Game/SurvivalGameKit/Blueprints/Other/Interfaces/BP_SurvivalInventoryInterface.Interact`
  (params (`Player Component` :type "/Game/SurvivalGameKit/Blueprints/Components/BP_PlayerInventoryComponent Object Reference"))
  ;[0 1 0.09084] Server events
  ;;[1 1 1] Server calls interact
  (`/Game/SurvivalGameKit/Blueprints/Components/BP_PlayerInventoryComponent.Server Pickup Item` `Player Component` self))

(event `self.ReceiveBeginPlay`
  (bind (_return_value _range_class) (`/Game/SurvivalGameKit/Blueprints/Other/Libraries/BP_InventoryFunctions.Range Weapon Details` (`self.Item`)))
  ;[0 0.5089 1] Client events
  ;;[1 1 1] Spawn attachments
  (`/Game/SurvivalGameKit/Blueprints/Other/Libraries/BP_InventoryMacros.IsItemWeapon?` (`self.Item`)
    (:`Weapon`
      (`SkinnedMeshComponent.SetSkinnedAssetAndUpdate` (`self.Skeletal World Mesh`) (`.EquippedMesh_92_18E57AC5491B8222B0CEE6AC4E6AC9A0` (break `/Game/SurvivalGameKit/Blueprints/Other/S_ItemDetails` (`.Item Details Out` (`/Game/SurvivalGameKit/Blueprints/Other/Libraries/BP_InventoryFunctions.Item Details` (`self.Item`))))) true)
      (if (`self.Player Dropped`)
        (`self.Server Spawn All Attachments` :!label _label)
        (elif _return_value
          (set `self.Attachments` (defaults `/Game/SurvivalGameKit/Blueprints/Items/BP_MasterItem` _range_class))
          (goto _label)
          (else
            (`self.Server Spawn All Attachments`)))))))

(event `Server Spawn All Attachments`
  ;[0 1 0.09084] Server events
  ;;[1 1 1] Server spawn all attachments
  (if (`KismetSystemLibrary.IsServer`)
    (`self.Spawn All Attachments`)))

(event `Destroy Item`
  ;[0 0.5089 1] Client events
  ;;[1 1 1] All clients destroy item
  (`self.Destroy All Attachments`)
  (`self.K2_DestroyActor`))

(fn `Destroy All Attachments`
  ;[1 1 1] Destroy all attachments
  (`self.Destroy Attachment` "NewEnumerator0")
  (`self.Destroy Attachment` "NewEnumerator1")
  (`self.Destroy Attachment` "NewEnumerator2")
  (`self.Destroy Attachment` "NewEnumerator3")
  (`self.Destroy Attachment` "NewEnumerator4")
  (`self.Destroy Attachment` "NewEnumerator5")
  (`self.Destroy Attachment` "NewEnumerator6")
  (`self.Destroy Attachment` "NewEnumerator7")
  (`self.Destroy Attachment` "NewEnumerator8"))

(fn `Destroy Attachment`
  (params (Attachment :type "/Game/SurvivalGameKit/Blueprints/Other/Enums/E_AttachmentType Enum" :default "NewEnumerator0") (`Remove Class` :type Boolean))
  (locals (`Attachment L` :type "/Game/SurvivalGameKit/Blueprints/Other/Enums/E_AttachmentType Enum" :default "NewEnumerator0") (`Remove Class L` :type Boolean))
  ;[1 1 1] Destroy attachment
  ;;[1 1 1] Switch on attachment
  (switch `/Game/SurvivalGameKit/Blueprints/Other/Enums/E_AttachmentType` (`local.Attachment`)
    (:`NewEnumerator0`
      ;;[1 1 1] Destroy actorand if remove class is true remove the attachment class from the attachments
      (`/Engine/EditorBlueprintResources/StandardMacros.IsValid` (`self.Sight`)
        (:`Is Valid`
          (`self.K2_DestroyActor` (`self.Sight`)))
        (:`Is Not Valid`
          _))
      (if (`local.Remove Class`)
        (bind _structout (setmembers `/Game/SurvivalGameKit/Blueprints/Other/S_WeaponAttachements` :`StructRef` (`self.Attachments`) :`Sight` null))
        (set `self.Attachments` _structout)))
    (:`NewEnumerator1`
      (`/Engine/EditorBlueprintResources/StandardMacros.IsValid` (`self.Front Grip`)
        (:`Is Valid`
          (`self.K2_DestroyActor` (`self.Front Grip`)))
        (:`Is Not Valid`
          _))
      (if (`local.Remove Class`)
        (bind _structout_2 (setmembers `/Game/SurvivalGameKit/Blueprints/Other/S_WeaponAttachements` :`StructRef` (`self.Attachments`) :`Front Grip` null))
        (set `self.Attachments` _structout_2)))
    (:`NewEnumerator2`
      (`/Engine/EditorBlueprintResources/StandardMacros.IsValid` (`self.Magazine`)
        (:`Is Valid`
          (`self.K2_DestroyActor` (`self.Magazine`)))
        (:`Is Not Valid`
          _))
      (if (`local.Remove Class`)
        (bind _structout_3 (setmembers `/Game/SurvivalGameKit/Blueprints/Other/S_WeaponAttachements` :`StructRef` (`self.Attachments`) :`Magazine` null))
        (set `self.Attachments` _structout_3)))
    (:`NewEnumerator3`
      (`/Engine/EditorBlueprintResources/StandardMacros.IsValid` (`self.Stock`)
        (:`Is Valid`
          (`self.K2_DestroyActor` (`self.Stock`)))
        (:`Is Not Valid`
          _))
      (if (`local.Remove Class`)
        (bind _structout_4 (setmembers `/Game/SurvivalGameKit/Blueprints/Other/S_WeaponAttachements` :`StructRef` (`self.Attachments`) :`Stock` null))
        (set `self.Attachments` _structout_4)))
    (:`NewEnumerator4`
      (`/Engine/EditorBlueprintResources/StandardMacros.IsValid` (`self.Trigger`)
        (:`Is Valid`
          (`self.K2_DestroyActor` (`self.Trigger`)))
        (:`Is Not Valid`
          _))
      (if (`local.Remove Class`)
        (bind _structout_5 (setmembers `/Game/SurvivalGameKit/Blueprints/Other/S_WeaponAttachements` :`StructRef` (`self.Attachments`) :`Trigger` null))
        (set `self.Attachments` _structout_5)))
    (:`NewEnumerator5`
      (`/Engine/EditorBlueprintResources/StandardMacros.IsValid` (`self.Handguard`)
        (:`Is Valid`
          (`self.K2_DestroyActor` (`self.Handguard`)))
        (:`Is Not Valid`
          _))
      (if (`local.Remove Class`)
        (bind _structout_6 (setmembers `/Game/SurvivalGameKit/Blueprints/Other/S_WeaponAttachements` :`StructRef` (`self.Attachments`) :`Handguard` null))
        (set `self.Attachments` _structout_6)))
    (:`NewEnumerator6`
      (`/Engine/EditorBlueprintResources/StandardMacros.IsValid` (`self.Underbarrel`)
        (:`Is Valid`
          (`self.K2_DestroyActor` (`self.Underbarrel`)))
        (:`Is Not Valid`
          _))
      (if (`local.Remove Class`)
        (bind _structout_7 (setmembers `/Game/SurvivalGameKit/Blueprints/Other/S_WeaponAttachements` :`StructRef` (`self.Attachments`) :`Handguard` null))
        (set `self.Attachments` _structout_7)))
    (:`NewEnumerator7`
      (`/Engine/EditorBlueprintResources/StandardMacros.IsValid` (`self.Muzzle`)
        (:`Is Valid`
          (`self.K2_DestroyActor` (`self.Muzzle`)))
        (:`Is Not Valid`
          _))
      (if (`local.Remove Class`)
        (bind _structout_8 (setmembers `/Game/SurvivalGameKit/Blueprints/Other/S_WeaponAttachements` :`StructRef` (`self.Attachments`) :`Muzzle` null))
        (set `self.Attachments` _structout_8)))
    (:`NewEnumerator8`
      (`/Engine/EditorBlueprintResources/StandardMacros.IsValid` (`self.Wrap`)
        (:`Is Valid`
          (`self.K2_DestroyActor` (`self.Wrap`)))
        (:`Is Not Valid`
          _))
      (if (`local.Remove Class`)
        (bind _structout_9 (setmembers `/Game/SurvivalGameKit/Blueprints/Other/S_WeaponAttachements` :`StructRef` (`self.Attachments`) :`Warp` null))
        (set `self.Attachments` _structout_9)))))

(fn `Interact Action`
  (returns (`Interact Action Text` :type Text))
  ;[1 1 1] Return action text (UI)
  (return "PICKUP"))

(fn `Interact Input Brush`
  (returns (Brush :type "SlateBrush Structure"))
  ;[1 1 1] Return the key icon (UI)
  (return (make `SlateBrush` (48.0 48.0) "Image" (struct) (struct :`SpecifiedColor` (struct :`R` 1.0 :`G` 1.0 :`B` 1.0 :`A` 1.0) :`ColorUseRule` "UseColor_Specified") "NoTile" "NoMirror" "/Game/SurvivalGameKit/Textures/UI/T_E_Interact.T_E_Interact")))

(fn `Interact Name`
  (returns (`Instace Text` :type Text))
  (return ""))

(fn `Interact Time`
  (returns (`Interact Time` :type Boolean) (Time :type "Float (double-precision)"))
  (bind ((`PickUpTime_146_A4405DC54967F650D060CFBCC6618430` _pickuptime)) (break `/Game/SurvivalGameKit/Blueprints/Other/S_ItemDetails` (`.Item Details Out` (`/Game/SurvivalGameKit/Blueprints/Other/Libraries/BP_InventoryFunctions.Item Details` (`self.Item`)))))
  ;[1 1 1] If > 0 return pick up time
  (return (> _pickuptime 0.0) _pickuptime))

(fn `Interacting Action Text`
  (returns (Text :type Text))
  ;[1 1 1] Set pick up time action text (UI)
  (return "COLLECTING"))

(fn `Is Interactable`
  (returns (Interactable :type Boolean))
  ;[1 1 1] Return if actor is interactable
  (return true))

(fn `Spawn All Attachments`
  (bind (_attachments_sight _attachments_frontgrip _attachments_magazine _attachments_stock _attachments_trigger _attachments_handguard _attachments_underbarrel _attachments_muzzle _attachments_warp) (break `/Game/SurvivalGameKit/Blueprints/Other/S_WeaponAttachements` (`self.Attachments`)))
  (bind _attachments_sight_2 (break `/Game/SurvivalGameKit/Blueprints/Other/S_WeaponAttachements` (`self.Attachments`)))
  (bind (_attachments_sight_3 _attachments_frontgrip_2) (break `/Game/SurvivalGameKit/Blueprints/Other/S_WeaponAttachements` (`self.Attachments`)))
  (bind (_attachments_sight_4 _attachments_frontgrip_3 _attachments_magazine_2) (break `/Game/SurvivalGameKit/Blueprints/Other/S_WeaponAttachements` (`self.Attachments`)))
  (bind (_attachments_sight_5 _attachments_frontgrip_4 _attachments_magazine_3 _attachments_stock_2) (break `/Game/SurvivalGameKit/Blueprints/Other/S_WeaponAttachements` (`self.Attachments`)))
  (bind (_attachments_sight_6 _attachments_frontgrip_5 _attachments_magazine_4 _attachments_stock_3 _attachments_trigger_2) (break `/Game/SurvivalGameKit/Blueprints/Other/S_WeaponAttachements` (`self.Attachments`)))
  (bind (_attachments_sight_7 _attachments_frontgrip_6 _attachments_magazine_5 _attachments_stock_4 _attachments_trigger_3 _attachments_handguard_2) (break `/Game/SurvivalGameKit/Blueprints/Other/S_WeaponAttachements` (`self.Attachments`)))
  (bind (_attachments_sight_8 _attachments_frontgrip_7 _attachments_magazine_6 _attachments_stock_5 _attachments_trigger_4 _attachments_handguard_3 _attachments_underbarrel_2) (break `/Game/SurvivalGameKit/Blueprints/Other/S_WeaponAttachements` (`self.Attachments`)))
  (bind (_attachments_sight_9 _attachments_frontgrip_8 _attachments_magazine_7 _attachments_stock_6 _attachments_trigger_5 _attachments_handguard_4 _attachments_underbarrel_3 _attachments_muzzle_2) (break `/Game/SurvivalGameKit/Blueprints/Other/S_WeaponAttachements` (`self.Attachments`)))
  ;[1 1 1] Spawn all attachments
  ;;[1 1 1] If attachment is valid spawn attachment actor
  (if (`KismetSystemLibrary.IsValidClass` _attachments_sight_2)
    (`self.Spawn Attachment` "NewEnumerator0"))
  ;;[1 1 1] If attachment is valid spawn attachment actor
  (if (`KismetSystemLibrary.IsValidClass` _attachments_frontgrip_2)
    (`self.Spawn Attachment` "NewEnumerator1"))
  ;;[1 1 1] If attachment is valid spawn attachment actor
  (if (`KismetSystemLibrary.IsValidClass` _attachments_magazine_2)
    (`self.Spawn Attachment` "NewEnumerator2"))
  ;;[1 1 1] If attachment is valid spawn attachment actor
  (if (`KismetSystemLibrary.IsValidClass` _attachments_stock_2)
    (`self.Spawn Attachment` "NewEnumerator3"))
  ;;[1 1 1] If attachment is valid spawn attachment actor
  (if (`KismetSystemLibrary.IsValidClass` _attachments_trigger_2)
    (`self.Spawn Attachment` "NewEnumerator4"))
  ;;[1 1 1] If attachment is valid spawn attachment actor
  (if (`KismetSystemLibrary.IsValidClass` _attachments_handguard_2)
    (`self.Spawn Attachment` "NewEnumerator5"))
  ;;[1 1 1] If attachment is valid spawn attachment actor
  (if (`KismetSystemLibrary.IsValidClass` _attachments_underbarrel_2)
    (`self.Spawn Attachment` "NewEnumerator6"))
  ;;[1 1 1] If attachment is valid spawn attachment actor
  (if (`KismetSystemLibrary.IsValidClass` _attachments_muzzle_2)
    (`self.Spawn Attachment` "NewEnumerator7"))
  ;;[1 1 1] If attachment is valid spawn attachment actor
  (if (`KismetSystemLibrary.IsValidClass` _attachments_warp)
    (`self.Spawn Attachment` "NewEnumerator8")))

(fn `Spawn Attachment`
  (params (Attachment :type "/Game/SurvivalGameKit/Blueprints/Other/Enums/E_AttachmentType Enum" :default "NewEnumerator0"))
  (locals (`Spawned Attachment L` :type "/Game/SurvivalGameKit/Blueprints/Attachments/BP_MasterAttachment Object Reference"))
  (bind (_attachments_sight _attachments_frontgrip _attachments_magazine _attachments_stock _attachments_trigger _attachments_handguard _attachments_underbarrel) (break `/Game/SurvivalGameKit/Blueprints/Other/S_WeaponAttachements` (`self.Attachments`)))
  (bind (_attachments_sight_2 _attachments_frontgrip_2 _attachments_magazine_2 _attachments_stock_2 _attachments_trigger_2) (break `/Game/SurvivalGameKit/Blueprints/Other/S_WeaponAttachements` (`self.Attachments`)))
  (bind (_attachments_sight_3 _attachments_frontgrip_3 _attachments_magazine_3 _attachments_stock_3 _attachments_trigger_3 _attachments_handguard_2) (break `/Game/SurvivalGameKit/Blueprints/Other/S_WeaponAttachements` (`self.Attachments`)))
  (bind _attachments_sight_4 (break `/Game/SurvivalGameKit/Blueprints/Other/S_WeaponAttachements` (`self.Attachments`)))
  (bind (_attachments_sight_5 _attachments_frontgrip_4) (break `/Game/SurvivalGameKit/Blueprints/Other/S_WeaponAttachements` (`self.Attachments`)))
  (bind (_attachments_sight_6 _attachments_frontgrip_5 _attachments_magazine_4) (break `/Game/SurvivalGameKit/Blueprints/Other/S_WeaponAttachements` (`self.Attachments`)))
  (bind (_attachments_sight_7 _attachments_frontgrip_6 _attachments_magazine_5 _attachments_stock_4) (break `/Game/SurvivalGameKit/Blueprints/Other/S_WeaponAttachements` (`self.Attachments`)))
  (bind (_attachments_sight_8 _attachments_frontgrip_7 _attachments_magazine_6 _attachments_stock_5 _attachments_trigger_4 _attachments_handguard_3 _attachments_underbarrel_2 _attachments_muzzle) (break `/Game/SurvivalGameKit/Blueprints/Other/S_WeaponAttachements` (`self.Attachments`)))
  (bind (_attachments_sight_9 _attachments_frontgrip_8 _attachments_magazine_7 _attachments_stock_6 _attachments_trigger_5 _attachments_handguard_4 _attachments_underbarrel_3 _attachments_muzzle_2 _attachments_warp) (break `/Game/SurvivalGameKit/Blueprints/Other/S_WeaponAttachements` (`self.Attachments`)))
  ;[1 1 1] Spawn attachment
  ;;[1 1 1] Is skeletal mesh valid
  (`/Engine/EditorBlueprintResources/StandardMacros.IsValid` (`self.Skeletal World Mesh`)
    (:`Is Valid`
      ;;[1 1 1] Switch on attachment
      (switch `/Game/SurvivalGameKit/Blueprints/Other/Enums/E_AttachmentType` (`local.Attachment`)
        (:`NewEnumerator0`
          ;;[1 1 1] Spawn sight attachment actor and attach to weapon socket
          (bind _returnvalue (`|SpawnActorFromClass` _attachments_sight_4 (`KismetMathLibrary.MakeTransform` (0.0 0.0 0.0)) "Undefined" "OverrideRootScale" null null))
          (bind _output_get (set `local.Spawned Attachment L` _returnvalue))
          (`self.K2_AttachToComponent` _output_get (`self.Skeletal World Mesh`) (`/Game/SurvivalGameKit/Blueprints/Attachments/BP_MasterAttachment.Attachment Socket Name` _returnvalue) "SnapToTarget" "SnapToTarget" "SnapToTarget" true)
          (set `self.Sight` (`local.Spawned Attachment L`)))
        (:`NewEnumerator1`
          ;;[1 1 1] Spawn front grip attachment actor and attach to weapon socket
          (bind _returnvalue_2 (`|SpawnActorFromClass` _attachments_frontgrip_4 (`KismetMathLibrary.MakeTransform` (0.0 0.0 0.0)) "Undefined" "OverrideRootScale" null null))
          (bind _output_get_2 (set `local.Spawned Attachment L` _returnvalue_2))
          (`self.K2_AttachToComponent` _output_get_2 (`self.Skeletal World Mesh`) (`/Game/SurvivalGameKit/Blueprints/Attachments/BP_MasterAttachment.Attachment Socket Name` _returnvalue_2) "SnapToTarget" "SnapToTarget" "SnapToTarget" true)
          (set `self.Front Grip` (`local.Spawned Attachment L`)))
        (:`NewEnumerator2`
          ;;[1 1 1] Spawn magazine attachment actor and attach to weapon socket
          (bind _returnvalue_3 (`|SpawnActorFromClass` _attachments_magazine_4 (`KismetMathLibrary.MakeTransform` (0.0 0.0 0.0)) "Undefined" "OverrideRootScale" null null))
          (bind _output_get_3 (set `local.Spawned Attachment L` _returnvalue_3))
          (`self.K2_AttachToComponent` _output_get_3 (`self.Skeletal World Mesh`) (`/Game/SurvivalGameKit/Blueprints/Attachments/BP_MasterAttachment.Attachment Socket Name` _returnvalue_3) "SnapToTarget" "SnapToTarget" "SnapToTarget" true)
          (set `self.Magazine` (`local.Spawned Attachment L`)))
        (:`NewEnumerator3`
          ;;[1 1 1] Spawn stock attachment actor and attach to weapon socket
          (bind _returnvalue_4 (`|SpawnActorFromClass` _attachments_stock_4 (`KismetMathLibrary.MakeTransform` (0.0 0.0 0.0)) "Undefined" "OverrideRootScale" null null))
          (bind _output_get_4 (set `local.Spawned Attachment L` _returnvalue_4))
          (`self.K2_AttachToComponent` _output_get_4 (`self.Skeletal World Mesh`) (`/Game/SurvivalGameKit/Blueprints/Attachments/BP_MasterAttachment.Attachment Socket Name` _returnvalue_4) "SnapToTarget" "SnapToTarget" "SnapToTarget" true)
          (set `self.Stock` (`local.Spawned Attachment L`)))
        (:`NewEnumerator4`
          ;;[1 1 1] Spawn trigger attachment actor and attach to weapon socket
          (bind _returnvalue_5 (`|SpawnActorFromClass` _attachments_trigger_2 (`KismetMathLibrary.MakeTransform` (0.0 0.0 0.0)) "Undefined" "OverrideRootScale" null null))
          (bind _output_get_5 (set `local.Spawned Attachment L` _returnvalue_5))
          (`self.K2_AttachToComponent` _output_get_5 (`self.Skeletal World Mesh`) (`/Game/SurvivalGameKit/Blueprints/Attachments/BP_MasterAttachment.Attachment Socket Name` _returnvalue_5) "SnapToTarget" "SnapToTarget" "SnapToTarget" true)
          (set `self.Trigger` (`local.Spawned Attachment L`)))
        (:`NewEnumerator5`
          ;;[1 1 1] Spawn handguard attachment actor and attach to weapon socket
          (bind _returnvalue_6 (`|SpawnActorFromClass` _attachments_handguard_2 (`KismetMathLibrary.MakeTransform` (0.0 0.0 0.0)) "Undefined" "OverrideRootScale" null null))
          (bind _output_get_6 (set `local.Spawned Attachment L` _returnvalue_6))
          (`self.K2_AttachToComponent` _output_get_6 (`self.Skeletal World Mesh`) (`/Game/SurvivalGameKit/Blueprints/Attachments/BP_MasterAttachment.Attachment Socket Name` _returnvalue_6) "SnapToTarget" "SnapToTarget" "SnapToTarget" true)
          (set `self.Handguard` (`local.Spawned Attachment L`)))
        (:`NewEnumerator6`
          ;;[1 1 1] Spawn underbarrel attachment actor and attach to weapon socket
          (bind _returnvalue_7 (`|SpawnActorFromClass` _attachments_underbarrel (`KismetMathLibrary.MakeTransform` (0.0 0.0 0.0)) "Undefined" "OverrideRootScale" null null))
          (bind _output_get_7 (set `local.Spawned Attachment L` _returnvalue_7))
          (`self.K2_AttachToComponent` _output_get_7 (`self.Skeletal World Mesh`) (`/Game/SurvivalGameKit/Blueprints/Attachments/BP_MasterAttachment.Attachment Socket Name` _returnvalue_7) "SnapToTarget" "SnapToTarget" "SnapToTarget" true)
          (set `self.Underbarrel` (`local.Spawned Attachment L`)))
        (:`NewEnumerator7`
          ;;[1 1 1] Spawn muzzle attachment actor and attach to weapon socket
          (bind _returnvalue_8 (`|SpawnActorFromClass` _attachments_muzzle (`KismetMathLibrary.MakeTransform` (0.0 0.0 0.0)) "Undefined" "OverrideRootScale" null null))
          (bind _output_get_8 (set `local.Spawned Attachment L` _returnvalue_8))
          (`self.K2_AttachToComponent` _output_get_8 (`self.Skeletal World Mesh`) (`/Game/SurvivalGameKit/Blueprints/Attachments/BP_MasterAttachment.Attachment Socket Name` _returnvalue_8) "SnapToTarget" "SnapToTarget" "SnapToTarget" true)
          (set `self.Muzzle` (`local.Spawned Attachment L`)))
        (:`NewEnumerator8`
          ;;[1 1 1] Spawn wrap attachment actor and attach to weapon socket
          (bind _returnvalue_9 (`|SpawnActorFromClass` _attachments_warp (`KismetMathLibrary.MakeTransform` (0.0 0.0 0.0)) "Undefined" "OverrideRootScale" null null))
          (bind _output_get_9 (set `local.Spawned Attachment L` _returnvalue_9))
          (`self.K2_AttachToComponent` _output_get_9 (`self.Skeletal World Mesh`) (`/Game/SurvivalGameKit/Blueprints/Attachments/BP_MasterAttachment.Attachment Socket Name` _returnvalue_9) "SnapToTarget" "SnapToTarget" "SnapToTarget" true)
          (set `self.Wrap` (`local.Spawned Attachment L`)))))))

(fn `UserConstructionScript`
  (bind (_select_item_datatable _select_item_rowname) (break `DataTableRowHandle` (`self.Select Item`)))
  (bind (_select_item_datatable_2 _select_item_rowname_2) (break `DataTableRowHandle` (`self.Select Item`)))
  (bind _item_id (break `/Game/SurvivalGameKit/Blueprints/Other/S_ItemInventory` (`self.Item`)))
  ;[1 1 1] Set up item
  (if (`/Game/SurvivalGameKit/Blueprints/Other/Libraries/BP_InventoryFunctions.Item Details` (make `/Game/SurvivalGameKit/Blueprints/Other/S_ItemInventory` (`KismetStringLibrary.Conv_NameToString` _select_item_rowname_2)))
    (set `self.Item` (make `/Game/SurvivalGameKit/Blueprints/Other/S_ItemInventory` (`KismetStringLibrary.Conv_NameToString` _select_item_rowname) (`self.Count`)))
    (else
      (set `self.Select Item` (make `DataTableRowHandle` "/Game/SurvivalGameKit/Blueprints/Items/ItemList.ItemList" (`KismetStringLibrary.Conv_StringToName` _item_id)))))
  (if (`/Game/SurvivalGameKit/Blueprints/Other/Libraries/BP_InventoryFunctions.Item Details` (`self.Item`))
    (`/Engine/EditorBlueprintResources/StandardMacros.IsValid` (`.EquippedMesh_92_18E57AC5491B8222B0CEE6AC4E6AC9A0` (break `/Game/SurvivalGameKit/Blueprints/Other/S_ItemDetails` (`.Item Details Out` (`/Game/SurvivalGameKit/Blueprints/Other/Libraries/BP_InventoryFunctions.Item Details` (`self.Item`)))))
      (:`Is Valid`
        (`/Game/SurvivalGameKit/Blueprints/Other/Libraries/BP_InventoryMacros.IsItemWeapon?` (`self.Item`)
          (:`Weapon`
            (`SkinnedMeshComponent.SetSkinnedAssetAndUpdate` (`self.Skeletal World Mesh`) (`.EquippedMesh_92_18E57AC5491B8222B0CEE6AC4E6AC9A0` (break `/Game/SurvivalGameKit/Blueprints/Other/S_ItemDetails` (`.Item Details Out` (`/Game/SurvivalGameKit/Blueprints/Other/Libraries/BP_InventoryFunctions.Item Details` (`self.Item`))))) true)
            (`StaticMeshComponent.SetStaticMesh` (`self.Static World Mesh`) null))
          (:`Not Weapon`
            (`StaticMeshComponent.SetStaticMesh` (`self.Static World Mesh`) (`.WorldMesh_59_7444C39B45931133AB5875A654072A5A` (break `/Game/SurvivalGameKit/Blueprints/Other/S_ItemDetails` (`.Item Details Out` (`/Game/SurvivalGameKit/Blueprints/Other/Libraries/BP_InventoryFunctions.Item Details` (`self.Item`))))) :!label _label))))
      (:`Is Not Valid`
        (goto _label)))
    (if (not (`self.Saved Loaded`))
      (`SceneComponent.K2_AddWorldTransform` (`self.Static World Mesh`) (`.MeshWorldOffset_122_C7831601440D7EC62305E8A0A25DF967` (break `/Game/SurvivalGameKit/Blueprints/Other/S_ItemDetails` (`.Item Details Out` (`/Game/SurvivalGameKit/Blueprints/Other/Libraries/BP_InventoryFunctions.Item Details` (`self.Item`))))) false false)
      (`SceneComponent.K2_AddWorldTransform` (`self.Skeletal World Mesh`) (`.MeshWorldOffset_122_C7831601440D7EC62305E8A0A25DF967` (break `/Game/SurvivalGameKit/Blueprints/Other/S_ItemDetails` (`.Item Details Out` (`/Game/SurvivalGameKit/Blueprints/Other/Libraries/BP_InventoryFunctions.Item Details` (`self.Item`))))) false false))))