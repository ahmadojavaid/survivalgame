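; Base weapon Blueprint for holdables, handling modular attachments, hitbox damage and the ADS camera.
; On spawn, the server validates each slot's class against the weapon, then multicasts spawning, which socket-attaches it, applies stats and caches it by type.
; Removal reverses stats and optionally updates the slot's class.
; Hitboxes come from component display names and select damage, with optional bleed; a fitted sight overrides the ADS camera transform.
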(event `On Spawned`
  ;[0 1 0.09084] Server events
  ;;[1 1 1] Spawn all attachments
  (`self.Server Spawn All Attachments`))

(event `/Game/SurvivalGameKit/Blueprints/Other/Interfaces/BP_SurvivalInventoryInterface.Remove Attachment`
  (params (Attachment :type "/Game/SurvivalGameKit/Blueprints/Other/Enums/E_AttachmentType Enum" :default "NewEnumerator0") (`Remove Class` :type Boolean))
  ;[0 1 0.09084] Server events
  ;;[1 1 1] Remove attachment
  (`self.Destroy Attachment` Attachment `Remove Class`))

(event `Server Spawn All Attachments`
  ;[0 1 0.09084] Server events
  ;;[1 1 1] Server spawn all attachments
  (`self.Add All Attachments`))

(event `Multicast Spawn Attachment`
  (params (Attachment :type "/Game/SurvivalGameKit/Blueprints/Attachments/BP_MasterAttachment Class Reference"))
  ;[1 0 0] Multicast events
  ;;[1 1 1] Multicast spawn new attachment
  (`self.Spawn Attachment` Attachment))

(event `/Game/SurvivalGameKit/Blueprints/Other/Interfaces/BP_SurvivalInventoryInterface.Add Attachment`
  (params (Attachment :type "/Game/SurvivalGameKit/Blueprints/Attachments/BP_MasterAttachment Class Reference"))
  ;[0 1 0.09084] Server events
  ;;[1 1 1] Interface calls to spawn attachment
  (`self.Multicast Spawn Attachment` Attachment))

(event `/Game/SurvivalGameKit/Blueprints/Other/Interfaces/BP_SurvivalInventoryInterface.Remove All Attachments`
  ;[0 1 0.09084] Server events
  ;;[1 1 1] Remove all attachments
  (`self.Destroy All Attachments`))

(fn `Add All Attachments`
  (bind _attachments_sight (break `/Game/SurvivalGameKit/Blueprints/Other/S_WeaponAttachements` (`self.Attachments`)))
  (bind _attachments_sight_2 (break `/Game/SurvivalGameKit/Blueprints/Other/S_WeaponAttachements` (`self.Attachments`)))
  (bind _attachments_sight_3 (break `/Game/SurvivalGameKit/Blueprints/Other/S_WeaponAttachements` (`self.Attachments`)))
  (bind (_attachments_sight_4 _attachments_frontgrip) (break `/Game/SurvivalGameKit/Blueprints/Other/S_WeaponAttachements` (`self.Attachments`)))
  (bind (_attachments_sight_5 _attachments_frontgrip_2) (break `/Game/SurvivalGameKit/Blueprints/Other/S_WeaponAttachements` (`self.Attachments`)))
  (bind (_attachments_sight_6 _attachments_frontgrip_3) (break `/Game/SurvivalGameKit/Blueprints/Other/S_WeaponAttachements` (`self.Attachments`)))
  (bind (_attachments_sight_7 _attachments_frontgrip_4 _attachments_magazine) (break `/Game/SurvivalGameKit/Blueprints/Other/S_WeaponAttachements` (`self.Attachments`)))
  (bind (_attachments_sight_8 _attachments_frontgrip_5 _attachments_magazine_2) (break `/Game/SurvivalGameKit/Blueprints/Other/S_WeaponAttachements` (`self.Attachments`)))
  (bind (_attachments_sight_9 _attachments_frontgrip_6 _attachments_magazine_3) (break `/Game/SurvivalGameKit/Blueprints/Other/S_WeaponAttachements` (`self.Attachments`)))
  (bind (_attachments_sight_10 _attachments_frontgrip_7 _attachments_magazine_4 _attachments_stock) (break `/Game/SurvivalGameKit/Blueprints/Other/S_WeaponAttachements` (`self.Attachments`)))
  (bind (_attachments_sight_11 _attachments_frontgrip_8 _attachments_magazine_5 _attachments_stock_2) (break `/Game/SurvivalGameKit/Blueprints/Other/S_WeaponAttachements` (`self.Attachments`)))
  (bind (_attachments_sight_12 _attachments_frontgrip_9 _attachments_magazine_6 _attachments_stock_3) (break `/Game/SurvivalGameKit/Blueprints/Other/S_WeaponAttachements` (`self.Attachments`)))
  (bind (_attachments_sight_13 _attachments_frontgrip_10 _attachments_magazine_7 _attachments_stock_4 _attachments_trigger) (break `/Game/SurvivalGameKit/Blueprints/Other/S_WeaponAttachements` (`self.Attachments`)))
  (bind (_attachments_sight_14 _attachments_frontgrip_11 _attachments_magazine_8 _attachments_stock_5 _attachments_trigger_2) (break `/Game/SurvivalGameKit/Blueprints/Other/S_WeaponAttachements` (`self.Attachments`)))
  (bind (_attachments_sight_15 _attachments_frontgrip_12 _attachments_magazine_9 _attachments_stock_6 _attachments_trigger_3) (break `/Game/SurvivalGameKit/Blueprints/Other/S_WeaponAttachements` (`self.Attachments`)))
  (bind (_attachments_sight_16 _attachments_frontgrip_13 _attachments_magazine_10 _attachments_stock_7 _attachments_trigger_4 _attachments_handguard) (break `/Game/SurvivalGameKit/Blueprints/Other/S_WeaponAttachements` (`self.Attachments`)))
  (bind (_attachments_sight_17 _attachments_frontgrip_14 _attachments_magazine_11 _attachments_stock_8 _attachments_trigger_5 _attachments_handguard_2) (break `/Game/SurvivalGameKit/Blueprints/Other/S_WeaponAttachements` (`self.Attachments`)))
  (bind (_attachments_sight_18 _attachments_frontgrip_15 _attachments_magazine_12 _attachments_stock_9 _attachments_trigger_6 _attachments_handguard_3) (break `/Game/SurvivalGameKit/Blueprints/Other/S_WeaponAttachements` (`self.Attachments`)))
  (bind (_attachments_sight_19 _attachments_frontgrip_16 _attachments_magazine_13 _attachments_stock_10 _attachments_trigger_7 _attachments_handguard_4 _attachments_underbarrel) (break `/Game/SurvivalGameKit/Blueprints/Other/S_WeaponAttachements` (`self.Attachments`)))
  (bind (_attachments_sight_20 _attachments_frontgrip_17 _attachments_magazine_14 _attachments_stock_11 _attachments_trigger_8 _attachments_handguard_5 _attachments_underbarrel_2) (break `/Game/SurvivalGameKit/Blueprints/Other/S_WeaponAttachements` (`self.Attachments`)))
  (bind (_attachments_sight_21 _attachments_frontgrip_18 _attachments_magazine_15 _attachments_stock_12 _attachments_trigger_9 _attachments_handguard_6 _attachments_underbarrel_3) (break `/Game/SurvivalGameKit/Blueprints/Other/S_WeaponAttachements` (`self.Attachments`)))
  (bind (_attachments_sight_22 _attachments_frontgrip_19 _attachments_magazine_16 _attachments_stock_13 _attachments_trigger_10 _attachments_handguard_7 _attachments_underbarrel_4 _attachments_muzzle) (break `/Game/SurvivalGameKit/Blueprints/Other/S_WeaponAttachements` (`self.Attachments`)))
  (bind (_attachments_sight_23 _attachments_frontgrip_20 _attachments_magazine_17 _attachments_stock_14 _attachments_trigger_11 _attachments_handguard_8 _attachments_underbarrel_5 _attachments_muzzle_2) (break `/Game/SurvivalGameKit/Blueprints/Other/S_WeaponAttachements` (`self.Attachments`)))
  (bind (_attachments_sight_24 _attachments_frontgrip_21 _attachments_magazine_18 _attachments_stock_15 _attachments_trigger_12 _attachments_handguard_9 _attachments_underbarrel_6 _attachments_muzzle_3) (break `/Game/SurvivalGameKit/Blueprints/Other/S_WeaponAttachements` (`self.Attachments`)))
  (bind (_attachments_sight_25 _attachments_frontgrip_22 _attachments_magazine_19 _attachments_stock_16 _attachments_trigger_13 _attachments_handguard_10 _attachments_underbarrel_7 _attachments_muzzle_4 _attachments_warp) (break `/Game/SurvivalGameKit/Blueprints/Other/S_WeaponAttachements` (`self.Attachments`)))
  (bind (_attachments_sight_26 _attachments_frontgrip_23 _attachments_magazine_20 _attachments_stock_17 _attachments_trigger_14 _attachments_handguard_11 _attachments_underbarrel_8 _attachments_muzzle_5 _attachments_warp_2) (break `/Game/SurvivalGameKit/Blueprints/Other/S_WeaponAttachements` (`self.Attachments`)))
  (bind (_attachments_sight_27 _attachments_frontgrip_24 _attachments_magazine_21 _attachments_stock_18 _attachments_trigger_15 _attachments_handguard_12 _attachments_underbarrel_9 _attachments_muzzle_6 _attachments_warp_3) (break `/Game/SurvivalGameKit/Blueprints/Other/S_WeaponAttachements` (`self.Attachments`)))
  ;[1 1 1] Add all attachments
  (if (`KismetSystemLibrary.IsValidClass` _attachments_sight)
    (bind _return_value (`/Game/SurvivalGameKit/Blueprints/Other/Libraries/BP_InventoryFunctions.Check Allowed Attachments` _attachments_sight_2 (`GameplayStatics.GetObjectClass` self)))
    (if _return_value
      (`self.Multicast Spawn Attachment` _attachments_sight_3)
      (if (`KismetSystemLibrary.IsValidClass` _attachments_frontgrip) :!label _label
        (bind _return_value_2 (`/Game/SurvivalGameKit/Blueprints/Other/Libraries/BP_InventoryFunctions.Check Allowed Attachments` _attachments_frontgrip_2 (`GameplayStatics.GetObjectClass` self)))
        (if _return_value_2
          (`self.Multicast Spawn Attachment` _attachments_frontgrip_3)
          (if (`KismetSystemLibrary.IsValidClass` _attachments_magazine) :!label _label_2
            (bind _return_value_3 (`/Game/SurvivalGameKit/Blueprints/Other/Libraries/BP_InventoryFunctions.Check Allowed Attachments` _attachments_magazine_2 (`GameplayStatics.GetObjectClass` self)))
            (if _return_value_3
              (`self.Multicast Spawn Attachment` _attachments_magazine_3)
              (if (`KismetSystemLibrary.IsValidClass` _attachments_stock) :!label _label_3
                (bind _return_value_4 (`/Game/SurvivalGameKit/Blueprints/Other/Libraries/BP_InventoryFunctions.Check Allowed Attachments` _attachments_stock_2 (`GameplayStatics.GetObjectClass` self)))
                (if _return_value_4
                  (`self.Multicast Spawn Attachment` _attachments_stock_3)
                  (if (`KismetSystemLibrary.IsValidClass` _attachments_trigger) :!label _label_4
                    (bind _return_value_5 (`/Game/SurvivalGameKit/Blueprints/Other/Libraries/BP_InventoryFunctions.Check Allowed Attachments` _attachments_trigger_2 (`GameplayStatics.GetObjectClass` self)))
                    (if _return_value_5
                      (`self.Multicast Spawn Attachment` _attachments_trigger_3)
                      (if (`KismetSystemLibrary.IsValidClass` _attachments_handguard) :!label _label_5
                        (bind _return_value_6 (`/Game/SurvivalGameKit/Blueprints/Other/Libraries/BP_InventoryFunctions.Check Allowed Attachments` _attachments_handguard_2 (`GameplayStatics.GetObjectClass` self)))
                        (if _return_value_6
                          (`self.Multicast Spawn Attachment` _attachments_handguard_3)
                          (if (`KismetSystemLibrary.IsValidClass` _attachments_underbarrel) :!label _label_6
                            (bind _return_value_7 (`/Game/SurvivalGameKit/Blueprints/Other/Libraries/BP_InventoryFunctions.Check Allowed Attachments` _attachments_underbarrel_2 (`GameplayStatics.GetObjectClass` self)))
                            (if _return_value_7
                              (`self.Multicast Spawn Attachment` _attachments_underbarrel_3)
                              (if (`KismetSystemLibrary.IsValidClass` _attachments_muzzle) :!label _label_7
                                (bind _return_value_8 (`/Game/SurvivalGameKit/Blueprints/Other/Libraries/BP_InventoryFunctions.Check Allowed Attachments` _attachments_muzzle_2 (`GameplayStatics.GetObjectClass` self)))
                                (if _return_value_8
                                  (`self.Multicast Spawn Attachment` _attachments_muzzle_3)
                                  (if (`KismetSystemLibrary.IsValidClass` _attachments_warp) :!label _label_8
                                    (bind _return_value_9 (`/Game/SurvivalGameKit/Blueprints/Other/Libraries/BP_InventoryFunctions.Check Allowed Attachments` _attachments_warp_2 (`GameplayStatics.GetObjectClass` self)))
                                    (if _return_value_9
                                      (`self.Multicast Spawn Attachment` _attachments_warp_3))))
                                (else
                                  (goto _label_8))))
                            (else
                              (goto _label_7))))
                        (else
                          (goto _label_6))))
                    (else
                      (goto _label_5))))
                (else
                  (goto _label_4))))
            (else
              (goto _label_3))))
        (else
          (goto _label_2))))
    (else
      (goto _label))))

(fn `Destroy All Attachments`
  ;[1 1 1] Destroy all attachments
  ;;[1 1 1] Loop through all attachments
  (for _array_element (`|MakeArray` "NewEnumerator0" "NewEnumerator1" "NewEnumerator2" "NewEnumerator3" "NewEnumerator4" "NewEnumerator5" "NewEnumerator6" "NewEnumerator7" "NewEnumerator8" :!type "/Game/SurvivalGameKit/Blueprints/Other/Enums/E_AttachmentType Enum")
    ;;[1 1 1] Destroy attachment
    (`self.Destroy Attachment` _array_element)))

(fn `Destroy Attachment`
  (params (Attachment :type "/Game/SurvivalGameKit/Blueprints/Other/Enums/E_AttachmentType Enum" :default "NewEnumerator0") (`Remove Class` :type Boolean))
  ;[1 1 1] Destroy attachment
  ;;[1 1 1] Get if there is a attachment of that type
  (if (`self.Get Attachment` (`local.Attachment`))
    ;;[1 1 1] Remove the attachments stats from weapon
    (`/Game/SurvivalGameKit/Blueprints/Other/Interfaces/BP_SurvivalInventoryInterface.Remove Attachment Stats` (`.Attachment` (`self.Get Attachment` (`local.Attachment`))) (`local.Remove Class`))
    ;;[1 1 1] Remove attachment class
    (if (`local.Remove Class`)
      ;;[1 1 1] Remove weapon class on switch
      (switch `/Game/SurvivalGameKit/Blueprints/Other/Enums/E_AttachmentType` (`local.Attachment`)
        (:`NewEnumerator0`
          (setmembers `/Game/SurvivalGameKit/Blueprints/Other/S_WeaponAttachements` :`StructRef` (`self.Attachments`) :`Sight` null))
        (:`NewEnumerator1`
          (setmembers `/Game/SurvivalGameKit/Blueprints/Other/S_WeaponAttachements` :`StructRef` (`self.Attachments`) :`Front Grip` null))
        (:`NewEnumerator2`
          (setmembers `/Game/SurvivalGameKit/Blueprints/Other/S_WeaponAttachements` :`StructRef` (`self.Attachments`) :`Magazine` null))
        (:`NewEnumerator3`
          (setmembers `/Game/SurvivalGameKit/Blueprints/Other/S_WeaponAttachements` :`StructRef` (`self.Attachments`) :`Stock` null))
        (:`NewEnumerator4`
          (setmembers `/Game/SurvivalGameKit/Blueprints/Other/S_WeaponAttachements` :`StructRef` (`self.Attachments`) :`Trigger` null))
        (:`NewEnumerator5`
          (setmembers `/Game/SurvivalGameKit/Blueprints/Other/S_WeaponAttachements` :`StructRef` (`self.Attachments`) :`Handguard` null))
        (:`NewEnumerator6`
          (setmembers `/Game/SurvivalGameKit/Blueprints/Other/S_WeaponAttachements` :`StructRef` (`self.Attachments`) :`Underbarrel` null))
        (:`NewEnumerator7`
          (setmembers `/Game/SurvivalGameKit/Blueprints/Other/S_WeaponAttachements` :`StructRef` (`self.Attachments`) :`Muzzle` null))
        (:`NewEnumerator8`
          (setmembers `/Game/SurvivalGameKit/Blueprints/Other/S_WeaponAttachements` :`StructRef` (`self.Attachments`) :`Warp` null))))))

(fn `Get Attachment`
  (params (`Attachment Type` :type "/Game/SurvivalGameKit/Blueprints/Other/Enums/E_AttachmentType Enum" :default "NewEnumerator0"))
  (returns (`Return Value` :type Boolean) (Attachment :type "/Game/SurvivalGameKit/Blueprints/Attachments/BP_MasterAttachment Object Reference"))
  (bind _returnvalue (select `/Game/SurvivalGameKit/Blueprints/Other/Enums/E_AttachmentType` (`local.Attachment Type`) :`NewEnumerator0` (`self.Sight`) :`NewEnumerator1` (`self.Front Grip`) :`NewEnumerator2` (`self.Magazine`) :`NewEnumerator3` (`self.Stock`) :`NewEnumerator4` (`self.Trigger`) :`NewEnumerator5` (`self.Handguard`) :`NewEnumerator6` (`self.Underbarrel`) :`NewEnumerator7` (`self.Muzzle`) :`NewEnumerator8` (`self.Warp`)))
  ;[1 1 1] Get attachment
  ;;[1 1 1] Is attachment actor valid
  (`/Engine/EditorBlueprintResources/StandardMacros.IsValid` _returnvalue
    (:`Is Valid`
      (return true _returnvalue))
    (:`Is Not Valid`
      (return false null))))

(fn `Return ADS Camera`
  (returns (`ADS Camera` :type "Transform Structure"))
  ;[1 1 1] Return ADS camera
  ;;[1 1 1] Is the sight valid
  (`/Engine/EditorBlueprintResources/StandardMacros.IsValid` (`self.Sight`)
    (:`Is Valid`
      ;;[1 1 1] Return camera transform from sight
      (return (`BlueprintMapLibrary.Map_Find` (`/Game/SurvivalGameKit/Blueprints/Attachments/BP_MasterAttachment.Camera Location` (`self.Sight`)) (`GameplayStatics.GetObjectClass` self))))
    (:`Is Not Valid`
      ;;[1 1 1] Return weapon camera transform
      (return (`self.Camera Location`)))))

(fn `Set Damage`
  (params (Hitbox :type "/Game/SurvivalGameKit/Blueprints/Other/Enums/E_HitboxType Enum" :default "NewEnumerator0") (`Hit Actor` :type "Actor Object Reference"))
  (locals (`Hitbox L` :type "/Game/SurvivalGameKit/Blueprints/Other/Enums/E_HitboxType Enum" :default "NewEnumerator0") (`Hit Actor L` :type "Actor Object Reference"))
  ;[1 1 1] Set damage
  ;;[1 1 1] Damage hit actor
  (message `/Game/SurvivalGameKit/Blueprints/Other/Interfaces/BP_SurvivalInventoryInterface.Damage` (`local.Hit Actor`) (`local.Hitbox`) (`BlueprintMapLibrary.Map_Find` (`self.Damage Values`) (`local.Hitbox`)))
  ;;[1 1 1] Does this weapon deal bleed damage
  (if (`self.Does Bleed Damage`)
    ;;[1 1 1] Apply bleed
    (message `/Game/SurvivalGameKit/Blueprints/Other/Interfaces/BP_SurvivalInventoryInterface.Bleed Damage` (`local.Hit Actor L`) (`self.Bleed Repeat Time`) (`self.Bleed Length`) (`self.Damage Per Bleed`))))

(fn `Set Hitbox`
  (params (Component :type "ActorComponent Object Reference"))
  (returns (Hitbox :type "/Game/SurvivalGameKit/Blueprints/Other/Enums/E_HitboxType Enum"))
  (locals (`Hitbox L` :type "/Game/SurvivalGameKit/Blueprints/Other/Enums/E_HitboxType Enum"))
  ;[1 1 1] Set hitbox
  ;;[1 1 1] Is the hitbox the head
  (if (`KismetStringLibrary.Contains` (`KismetSystemLibrary.GetDisplayName` (`local.Component`)) "HeadHitbox")
    (bind _output_get (set `local.Hitbox L` "NewEnumerator1"))
    (return _output_get)
    (else
      ;;[1 1 1] Is the hitbox the arm
      (if (`KismetStringLibrary.Contains` (`KismetSystemLibrary.GetDisplayName` (`local.Component`)) "ArmHitbox")
        (bind _output_get_2 (set `local.Hitbox L` "NewEnumerator3"))
        (return _output_get_2)
        (else
          ;;[1 1 1] Is the hitbox the chest
          (if (`KismetStringLibrary.Contains` (`KismetSystemLibrary.GetDisplayName` (`local.Component`)) "ChestHitbox")
            (bind _output_get_3 (set `local.Hitbox L` "NewEnumerator2"))
            (return _output_get_3)
            (else
              ;;[1 1 1] Is the hitbox the leg
              (if (`KismetStringLibrary.Contains` (`KismetSystemLibrary.GetDisplayName` (`local.Component`)) "LegHitbox")
                (bind _output_get_4 (set `local.Hitbox L` "NewEnumerator4"))
                (return _output_get_4)
                (else
                  (bind _output_get_5 (set `local.Hitbox L` "NewEnumerator0"))
                  (return _output_get_5))))))))))

(fn `Spawn Attachment`
  (params (Attachment :type "/Game/SurvivalGameKit/Blueprints/Attachments/BP_MasterAttachment Class Reference"))
  (locals (`Spawned Attachment L` :type "/Game/SurvivalGameKit/Blueprints/Attachments/BP_MasterAttachment Object Reference"))
  (bind (_returnvalue_location _returnvalue_rotation) (`KismetMathLibrary.BreakTransform` (`SceneComponent.GetSocketTransform` (`self.Weapon Skeletal Mesh`) (defaults `/Game/SurvivalGameKit/Blueprints/Holdables/BP_MasterWeapon` (`local.Attachment`)) "RTS_World")))
  ;[1 1 1] Spawn attachment
  ;;[1 1 1] Is valid
  (if (`KismetSystemLibrary.IsValidClass` (`local.Attachment`))
    ;;[1 1 1] Spawn attachment at socket location
    (bind _returnvalue (`|SpawnActorFromClass` (`local.Attachment`) (`KismetMathLibrary.MakeTransform` _returnvalue_location _returnvalue_rotation) "AlwaysSpawn" "OverrideRootScale" null null))
    (bind _output_get (set `local.Spawned Attachment L` _returnvalue))
    ;;[1 1 1] Attach actor to socket
    (`self.K2_AttachToComponent` _output_get (`self.Weapon Skeletal Mesh`) (`/Game/SurvivalGameKit/Blueprints/Attachments/BP_MasterAttachment.Attachment Socket Name` _output_get) "SnapToTarget" "SnapToTarget" "SnapToTarget" true)
    ;;[1 1 1] Add attachment stats
    (message `/Game/SurvivalGameKit/Blueprints/Other/Interfaces/BP_SurvivalInventoryInterface.Add Attachment Stats` self (`local.Spawned Attachment L`))
    ;;[1 1 1] Set actors reference using switch
    (switch `/Game/SurvivalGameKit/Blueprints/Other/Enums/E_AttachmentType` (`/Game/SurvivalGameKit/Blueprints/Attachments/BP_MasterAttachment.Attachment Type` (`local.Spawned Attachment L`))
      (:`NewEnumerator0`
        (set `self.Sight` (`local.Spawned Attachment L`)))
      (:`NewEnumerator1`
        (set `self.Front Grip` (`local.Spawned Attachment L`)))
      (:`NewEnumerator2`
        (set `self.Magazine` (`local.Spawned Attachment L`)))
      (:`NewEnumerator3`
        (set `self.Stock` (`local.Spawned Attachment L`)))
      (:`NewEnumerator4`
        (set `self.Trigger` (`local.Spawned Attachment L`)))
      (:`NewEnumerator5`
        (set `self.Handguard` (`local.Spawned Attachment L`)))
      (:`NewEnumerator6`
        (set `self.Underbarrel` (`local.Spawned Attachment L`)))
      (:`NewEnumerator7`
        (set `self.Muzzle` (`local.Spawned Attachment L`)))
      (:`NewEnumerator8`
        (set `self.Warp` (`local.Spawned Attachment L`))))))

(fn `UserConstructionScript`
  (`parent.UserConstructionScript`))