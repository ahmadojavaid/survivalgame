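; BP_MasterHoldable is a base Blueprint for holdable items in the Survival Game Kit.
; Its Destroy event, grouped under server events, sends a Remove All Attachments message before destroying the actor.
; It implements interaction query functions with empty defaults, reporting itself as non-interactable with no timed interaction.
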(event `Destroy`
  ;[0 1 0.09084] Server events
  ;;[1 1 1] Destroy this actor
  (message `/Game/SurvivalGameKit/Blueprints/Other/Interfaces/BP_SurvivalInventoryInterface.Remove All Attachments` self)
  (`self.K2_DestroyActor`))

(fn `Interact Action`
  (returns (`Interact Action Text` :type Text))
  (return ""))

(fn `Interact Input Brush`
  (returns (Brush :type "SlateBrush Structure"))
  (return))

(fn `Interact Name`
  (returns (`Instace Text` :type Text))
  (return ""))

(fn `Interact Time`
  (returns (`Interact Time` :type Boolean) (Time :type "Float (double-precision)"))
  (return false 0.0))

(fn `Interacting Action Text`
  (returns (Text :type Text))
  (return ""))

(fn `Is Interactable`
  (returns (Interactable :type Boolean))
  (return false))

(fn `UserConstructionScript`)