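; Base survival-kit character with modular body meshes, first/third-person cameras, weapon ADS zoom and recoil, and stubbed interaction functions.
; Damage and bleeding forward to PlayerInventoryComponent, and server-timed falls past a velocity threshold deduct health.
; Camera switches toggle owner mesh visibility and reattach the held item, while timelines blend first-person ADS.
; Tick relays look and actor rotation through server/multicast events and turns the body once control yaw diverges 80 degrees.
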(event `Destroy Character`
  (params (Timer :type "Float (double-precision)"))
  (bind _held_actor (`self.Held Actor`))
  ;[0 1 0.09084] Server events
  ;;[1 1 1] Kill character
  (`KismetSystemLibrary.Delay` Timer)
  (`/Engine/EditorBlueprintResources/StandardMacros.IsValid` _held_actor
    (:`Is Valid`
      (`self.K2_DestroyActor` _held_actor))
    (:`Is Not Valid`
      _))
  (`self.K2_DestroyActor`))

(event `/Game/SurvivalGameKit/Blueprints/Other/Interfaces/BP_SurvivalInventoryInterface.Bleed Damage`
  (params (`Bleed Repeat Time` :type "Float (single-precision)") (`Bleed Length` :type "Float (single-precision)") (`Bleed Damage` :type Integer))
  ;[0 1 0.09084] Server events
  ;;[1 1 1] Bleed damage
  (`/Game/SurvivalGameKit/Blueprints/Other/Interfaces/BP_SurvivalInventoryInterface.Bleed Damage` (`self.PlayerInventoryComponent`) `Bleed Repeat Time` `Bleed Length` `Bleed Damage`))

(event `self.OnLanded`
  (params (Hit :type "HitResult Structure (by ref)"))
  ;[0 1 0.09084] Server events
  ;;[1 1 1] On landed
  (if (`self.Fall Damage `)
    (if (`self.Damage Velocity Reached`)
      (set `self.End Fall Time` (`GameplayStatics.GetRealTimeSeconds`))
      (if (> (- (`self.End Fall Time`) (`self.Start Fall Time`)) (`self.Start Fall Damage Time`))
        (`/Game/SurvivalGameKit/Blueprints/Components/BP_PlayerInventoryComponent.Deduct Health` (`self.PlayerInventoryComponent`) (`KismetMathLibrary.FTrunc` (* (`.ReturnValue` (`KismetMathLibrary.FMod` (- (`self.End Fall Time`) (`self.Start Fall Time`)) (`self.Fall Damage Increese Time`))) (`self.Fall Damage`))))
        (`self.Reset Fall Damage`)
        (else
          (`self.Reset Fall Damage`))))))

(event `/Game/SurvivalGameKit/Blueprints/Other/Interfaces/BP_SurvivalInventoryInterface.Damage`
  (params (Hitbox :type "/Game/SurvivalGameKit/Blueprints/Other/Enums/E_HitboxType Enum" :default "NewEnumerator0") (Damage :type Integer))
  ;[0 1 0.09084] Server events
  ;;[1 1 1] Damage
  (`/Game/SurvivalGameKit/Blueprints/Other/Interfaces/BP_SurvivalInventoryInterface.Damage` (`self.PlayerInventoryComponent`) Hitbox Damage))

(event `Multicast Stop Character Movement`
  ;[1 0 0] Multicast events
  ;;[1 1 1] Multicast stop character movement
  (`MovementComponent.StopMovementImmediately` (`self.CharacterMovement`)))

(event `Third Person`
  (bind _asbp_master_holdable (cast `/Game/SurvivalGameKit/Blueprints/Holdables/BP_MasterHoldable` (`self.Held Actor`) :!pure true))
  ;[0 0.5089 1] Client events
  ;;[1 1 1] Client third person camera
  (`/Game/SurvivalGameKit/Blueprints/Components/BP_PlayerInventoryComponent.Client Camera View` (`self.PlayerInventoryComponent`) "NewEnumerator1")
  (set `self.Camera View` "NewEnumerator1")
  (`ActorComponent.Deactivate` (`self.FP Camera`))
  (`ActorComponent.Activate` (`self.TP Camera`) true)
  (`PrimitiveComponent.SetOwnerNoSee` (`self.Head`) false)
  (`PrimitiveComponent.SetOwnerNoSee` (`self.Legs`) false)
  (`PrimitiveComponent.SetOwnerNoSee` (`self.Backpack`) false)
  (`PrimitiveComponent.SetOwnerNoSee` (`self.Feet`) false)
  (`PrimitiveComponent.SetOwnerNoSee` (`self.Chest`) false)
  (`PrimitiveComponent.SetOwnerNoSee` (`self.Mesh`) false)
  (`SceneComponent.SetVisibility` (`self.FP Viewport Mesh`) false false)
  (`/Engine/EditorBlueprintResources/StandardMacros.IsValid` (`self.Held Actor`)
    (:`Is Valid`
      (`SceneComponent.K2_AttachToComponent` (`/Game/SurvivalGameKit/Blueprints/Holdables/BP_MasterHoldable.Attach Component` _asbp_master_holdable) (`self.Mesh`) (`/Game/SurvivalGameKit/Blueprints/Holdables/BP_MasterHoldable.Socket Name` _asbp_master_holdable) "SnapToTarget" "SnapToTarget" "SnapToTarget" true))))

(event `First Person`
  (bind _asbp_master_holdable (cast `/Game/SurvivalGameKit/Blueprints/Holdables/BP_MasterHoldable` (`self.Held Actor`) :!pure true))
  ;[0 0.5089 1] Client events
  ;;[1 1 1] Client first person camera
  (`/Game/SurvivalGameKit/Blueprints/Components/BP_PlayerInventoryComponent.Client Camera View` (`self.PlayerInventoryComponent`) "NewEnumerator0")
  (set `self.Camera View` "NewEnumerator0")
  (`ActorComponent.Deactivate` (`self.TP Camera`))
  (`ActorComponent.Activate` (`self.FP Camera`) true)
  (`PrimitiveComponent.SetOwnerNoSee` (`self.Head`) true)
  (`PrimitiveComponent.SetOwnerNoSee` (`self.Legs`) true)
  (`PrimitiveComponent.SetOwnerNoSee` (`self.Backpack`) true)
  (`PrimitiveComponent.SetOwnerNoSee` (`self.Feet`) true)
  (`PrimitiveComponent.SetOwnerNoSee` (`self.Chest`) true)
  (`PrimitiveComponent.SetOwnerNoSee` (`self.Mesh`) true)
  (`SceneComponent.SetVisibility` (`self.FP Viewport Mesh`) true false)
  (`/Engine/EditorBlueprintResources/StandardMacros.IsValid` (`self.Held Actor`)
    (:`Is Valid`
      (`self.K2_DetachFromActor` (`self.Held Actor`) "KeepRelative" "KeepRelative" "KeepRelative")
      (`SceneComponent.K2_AttachToComponent` (`/Game/SurvivalGameKit/Blueprints/Holdables/BP_MasterHoldable.Attach Component` _asbp_master_holdable) (`self.FP Viewport Mesh`) (`/Game/SurvivalGameKit/Blueprints/Holdables/BP_MasterHoldable.Socket Name` _asbp_master_holdable) "SnapToTarget" "SnapToTarget" "SnapToTarget" true))))

(event `Reset Fall Damage`
  ;[0 0.5089 1] Client events
  ;;[1 1 1] Set all character rotations
  (set `self.Start Fall Time` 0.0)
  (set `self.End Fall Time` 0.0)
  (set `self.Damage Velocity Reached` false)
  (goto _label :!via `Reset`))

(event `self.ReceiveBeginPlay`
  ;[0 1 0.09084] Server events
  ;;[1 1 1] Begin play
  (set `/Game/SurvivalGameKit/Blueprints/Components/BP_PlayerInventoryComponent.Player Building Component` (`self.PlayerBuildingComponent`) (`self.PlayerInventoryComponent`))
  (if (`|EnumEquality` (`self.Camera View`) "NewEnumerator0")
    (`self.First Person`)))

(event `self.ReceiveTick`
  (params (DeltaSeconds :type "Float (single-precision)"))
  (bind (_returnvalue_roll _returnvalue_pitch _returnvalue_yaw) (`KismetMathLibrary.BreakRotator` (`self.K2_GetActorRotation`)))
  (bind (_returnvalue_roll_2 _returnvalue_pitch_2 _returnvalue_yaw_2) (`KismetMathLibrary.BreakRotator` (`self.GetControlRotation`)))
  (bind (_returnvalue_roll_3 _returnvalue_pitch_3 _returnvalue_yaw_3) (`KismetMathLibrary.BreakRotator` (`KismetMathLibrary.NormalizedDeltaRotator` (`KismetMathLibrary.MakeRotator` 0.0 0.0 _returnvalue_yaw_2) (`KismetMathLibrary.MakeRotator` 0.0 0.0 _returnvalue_yaw))))
  (bind (_velocity_x _velocity_y _velocity_z) (`KismetMathLibrary.BreakVector` (`MovementComponent.Velocity` (`self.CharacterMovement`))))
  ;[0 0.5089 1] Client events
  ;;[1 1 1] Set all character rotations
  (`|ExecutionSequence`
    (:`then_0`
      (`/Engine/EditorBlueprintResources/ActorMacros.Switch Has Authority`
        (:`Authority`
          (if (`self.IsLocallyControlled`)
            (`self.Multicast Look At Rotation` (`self.GetControlRotation`))
            (set `self.Look At Rotation` (`self.GetControlRotation`))))
        (:`Remote`
          (`/Engine/EditorBlueprintResources/StandardMacros.IsValid` (`self.GetController`)
            (:`Is Valid`
              (`self.Server Look At Rotation` (`self.GetControlRotation`))
              (set `self.Look At Rotation` (`self.GetControlRotation`)))))))
    (:`then_1`
      (if (or (`self.Rotate Character`) (>= (`KismetMathLibrary.Abs` _returnvalue_yaw_3) 80.0))
        (set `CharacterMovementComponent.bUseControllerDesiredRotation` true (`self.CharacterMovement`))
        (set `self.Rotate Character` (not (`KismetMathLibrary.NearlyEqual_FloatFloat` _returnvalue_yaw_3 0.0 2.0)))
        (else
          (set `CharacterMovementComponent.bUseControllerDesiredRotation` false (`self.CharacterMovement`)))))
    (:`then_2`
      (`/Engine/EditorBlueprintResources/ActorMacros.Switch Has Authority`
        (:`Authority`
          (if (`self.IsLocallyControlled`)
            (`self.Multicast Actor Rotation` (`self.K2_GetActorRotation`))
            (`self.K2_SetActorRotation` (`self.K2_GetActorRotation`))))
        (:`Remote`
          (`/Engine/EditorBlueprintResources/StandardMacros.IsValid` (`self.GetController`)
            (:`Is Valid`
              (`self.Server Actor Rotation` (`self.K2_GetActorRotation`))
              (`self.K2_SetActorRotation` (`self.K2_GetActorRotation`)))))))
    (:`then_3`
      (if (`self.Fall Damage `)
        (`/Engine/EditorBlueprintResources/ActorMacros.Switch Has Authority`
          (:`Authority`
            (if (`NavMovementComponent.IsFalling` (`self.CharacterMovement`))
              (if (<= _velocity_z (`self.Fall Damage Velocity`))
                (set `self.Damage Velocity Reached` true)
                (`/Engine/EditorBlueprintResources/StandardMacros.DoOnce` false :!label _label
                  (:`Completed`
                    (set `self.Start Fall Time` (`GameplayStatics.GetRealTimeSeconds`))))))))))))

(event `Server Look At Rotation`
  (params (Rotation :type "Rotator Structure"))
  ;[0 1 0.09084] Server events
  ;;[1 1 1] Server look at rotation
  (`self.Multicast Look At Rotation` Rotation))

(event `Multicast Look At Rotation`
  (params (Rotation :type "Rotator Structure"))
  ;[1 0 0] Multicast events
  ;;[1 1 1] Multicast look at rotation
  (set `self.Look At Rotation` Rotation))

(event `Server Actor Rotation`
  (params (Rotation :type "Rotator Structure"))
  ;[0 1 0.09084] Server events
  ;;[1 1 1] Server actor rotation
  (`self.Multicast Actor Rotation` Rotation))

(event `Client Set Speed`
  (params (Speed :type "Float (double-precision)"))
  ;[0 0.5089 1] Client events
  ;;[1 1 1] Client set character speed
  (set `CharacterMovementComponent.MaxWalkSpeed` Speed (`self.CharacterMovement`)))

(event `Multicast Actor Rotation`
  (params (Rotation :type "Rotator Structure"))
  ;[1 0 0] Multicast events
  ;;[1 1 1] Multicast actor rotation
  (if (`self.IsLocallyControlled`)
    (if (not (`|EnumEquality` (`self.Camera View`) "NewEnumerator0"))
      (`self.K2_SetActorRotation` Rotation :!label _label_2))
    (else
      (goto _label_2))))

(event `Client Recoil`
  (params (`Weapon Recoil` :type "/Game/SurvivalGameKit/Blueprints/Other/S_WeaponRecoil Structure"))
  (bind (_yawmin _yawmax _pitchmin _pitchmax) (break `/Game/SurvivalGameKit/Blueprints/Other/S_WeaponRecoil` `Weapon Recoil`))
  ;[0 0.5089 1] Client events
  ;;[1 1 1] Client recoil
  (`self.AddControllerYawInput` (`KismetMathLibrary.RandomFloatInRange` _yawmin _yawmax))
  (`self.AddControllerPitchInput` (`KismetMathLibrary.RandomFloatInRange` _pitchmin _pitchmax)))

(event `Client Zoom In ADS`
  ;[0 0.5089 1] Client events
  ;;[1 1 1] Client zoom In ADS
  (`SceneComponent.K2_SetRelativeTransform` (`self.ADS Socket`) (`/Game/SurvivalGameKit/Blueprints/Holdables/BP_MasterWeapon.Return ADS Camera` (cast `/Game/SurvivalGameKit/Blueprints/Holdables/BP_MasterWeapon` (`self.Held Actor`) :!pure true)) false false)
  (`ActorComponent.Deactivate` (`self.FP Camera`))
  (if (`/Game/SurvivalGameKit/Blueprints/Components/BP_PlayerInventoryComponent.Was Third Person` (`self.PlayerInventoryComponent`))
    (`ActorComponent.Activate` (`self.ADS Camera`) true)
    (set `self.Camera Animation` false)
    (`SceneComponent.K2_SetWorldTransform` (`self.ADS Camera`) (`SceneComponent.K2_GetComponentToWorld` (`self.ADS Socket`)) false false)
    (`SceneComponent.K2_AttachToComponent` (`self.ADS Camera`) (`self.ADS Socket`) "None" "SnapToTarget" "SnapToTarget" "SnapToTarget" true)
    (`CameraComponent.SetFieldOfView` (`self.ADS Camera`) (`/Game/SurvivalGameKit/Blueprints/Holdables/BP_MasterRangeWeapon.ADS FOV` (cast `/Game/SurvivalGameKit/Blueprints/Holdables/BP_MasterRangeWeapon` (`self.Held Actor`) :!pure true)))
    (if (`/Game/SurvivalGameKit/Blueprints/Components/BP_PlayerInventoryComponent.Equipping` (`self.PlayerInventoryComponent`))
      (`/Game/SurvivalGameKit/Blueprints/Components/BP_PlayerInventoryComponent.Client Exit Aimed` (`self.PlayerInventoryComponent`) true))
    (else
      (`ActorComponent.Activate` (`self.ADS Camera`) true)
      (set `self.Camera Animation` true)
      (bind (_direction _zoom_in) (`Timeline|Zoom In` :!via `PlayFromStart` :!label _label_3)
        (:`Update`
          (if (`/Game/SurvivalGameKit/Blueprints/Components/BP_PlayerInventoryComponent.Equipping` (`self.PlayerInventoryComponent`))
            (`|ExecutionSequence`
              (:`then_0`
                (`self.Stop FP Zoom In ADS`))
              (:`then_1`
                (`/Game/SurvivalGameKit/Blueprints/Components/BP_PlayerInventoryComponent.Client Exit Aimed` (`self.PlayerInventoryComponent`) true)))
            (else
              (`SceneComponent.K2_SetWorldTransform` (`self.ADS Camera`) (`KismetMathLibrary.TLerp` (`SceneComponent.K2_GetComponentToWorld` (`self.ADS Camera`)) (`SceneComponent.K2_GetComponentToWorld` (`self.ADS Socket`)) _zoom_in) false false)
              (`CameraComponent.SetFieldOfView` (`self.ADS Camera`) (`KismetMathLibrary.Lerp` 90.0 (`/Game/SurvivalGameKit/Blueprints/Holdables/BP_MasterRangeWeapon.ADS FOV` (cast `/Game/SurvivalGameKit/Blueprints/Holdables/BP_MasterRangeWeapon` (`self.Held Actor`) :!pure true)) _zoom_in)))))
        (:`Finished`
          (set `self.Camera Animation` false)
          (`SceneComponent.K2_AttachToComponent` (`self.ADS Camera`) (`self.ADS Socket`) "None" "SnapToTarget" "SnapToTarget" "SnapToTarget" true))))))

(event `Stop FP Zoom In ADS`
  ;[0 0.5089 1] Client events
  ;;[1 1 1] Client zoom In ADS
  (goto _label_3 :!via `Stop`))

(event `Client Zoom Out ADS`
  ;[0 0.5089 1] Client events
  ;;[1 1 1] Client zoom out ADS
  (if (`/Game/SurvivalGameKit/Blueprints/Components/BP_PlayerInventoryComponent.Was Third Person` (`self.PlayerInventoryComponent`))
    (`SceneComponent.K2_SetWorldTransform` (`self.ADS Camera`) (`SceneComponent.K2_GetComponentToWorld` (`self.FP Camera`)) false false)
    (set `self.Camera Animation` false)
    (`ActorComponent.Deactivate` (`self.ADS Camera`))
    (if (`/Game/SurvivalGameKit/Blueprints/Components/BP_PlayerInventoryComponent.Was Third Person` (`self.PlayerInventoryComponent`))
      (`self.Third Person`)
      (else
        (`self.First Person`)))
    (else
      (set `self.Camera Animation` true)
      (bind (_direction _zoom_out) (`Timeline|Zoom Out` :!via `PlayFromStart`)
        (:`Update`
          (`CameraComponent.SetFieldOfView` (`self.ADS Camera`) (`KismetMathLibrary.Lerp` 75.0 90.0 _zoom_out))
          (`SceneComponent.K2_SetWorldTransform` (`self.ADS Camera`) (`KismetMathLibrary.TLerp` (`SceneComponent.K2_GetComponentToWorld` (`self.ADS Camera`)) (`SceneComponent.K2_GetComponentToWorld` (`self.FP Camera`)) _zoom_out) false false))
        (:`Finished`
          (set `self.Camera Animation` false)
          (`ActorComponent.Deactivate` (`self.ADS Camera`))
          (if (`/Game/SurvivalGameKit/Blueprints/Components/BP_PlayerInventoryComponent.Was Third Person` (`self.PlayerInventoryComponent`))
            (`self.Third Person`)
            (else
              (`self.First Person`))))))))

(fn `Interact Action`
  (returns (`Interact Action Text` :type Text))
  (return ""))

(fn `Interact Input Brush`
  (returns (Brush :type "SlateBrush Structure"))
  (return))

(fn `Interact Name`
  (returns (`Instace Text` :type Text))
  (return ""))

(fn `Interact Time`
  (returns (`Interact Time` :type Boolean) (Time :type "Float (double-precision)"))
  (return false 0.0))

(fn `Interacting Action Text`
  (returns (Text :type Text))
  (return ""))

(fn `Is Interactable`
  (returns (Interactable :type Boolean))
  (return false))

(fn `UserConstructionScript`
  (`SkinnedMeshComponent.SetLeaderPoseComponent` (`self.Head`) (`self.Mesh`))
  (`SkinnedMeshComponent.SetLeaderPoseComponent` (`self.Backpack`) (`self.Mesh`))
  (`SkinnedMeshComponent.SetLeaderPoseComponent` (`self.Chest`) (`self.Mesh`))
  (`SkinnedMeshComponent.SetLeaderPoseComponent` (`self.Legs`) (`self.Mesh`))
  (`SkinnedMeshComponent.SetLeaderPoseComponent` (`self.Feet`) (`self.Mesh`)))