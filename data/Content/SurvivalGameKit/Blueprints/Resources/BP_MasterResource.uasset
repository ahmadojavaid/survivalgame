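; BP_MasterResource is the base harvestable resource actor, holding an item row and remaining count.
; ResourceCollected multicasts a hit sound at the actor, subtracts the requested amount, destroys the actor at zero, and returns item ID and amount.
; When the request exceeds the stock, it returns the remaining count without decrementing or destroying the actor.
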(event `Multicast Play Hit Sound`
  ;[1 1 1] Multicast events
  ;;[1 1 1] Multicast play hit sound
  (`GameplayStatics.PlaySoundAtLocation` (`self.Hit Sound`) (`self.K2_GetActorLocation`) (struct) 1.0 1.0 0.0 "/Game/SurvivalGameKit/Sounds/CampFire.CampFire"))

(fn `Resource Collected`
  (params (`Collected Amount` :type Integer))
  (returns (Item :type "/Game/SurvivalGameKit/Blueprints/Other/S_ItemInventory Structure"))
  (locals (`Harvested Amount L` :type Integer))
  (bind (_item _count) (break `/Game/SurvivalGameKit/Blueprints/Other/S_Item` (`self.Item`)))
  (bind (_item_2 _count_2) (break `/Game/SurvivalGameKit/Blueprints/Other/S_Item` (`self.Item`)))
  (set `local.Harvested Amount L` `Collected Amount`)
  (`self.Multicast Play Hit Sound`)
  (if (> (`.Count_8_4FA908A94D8A3E10DFE8349075F8DC5E` (break `/Game/SurvivalGameKit/Blueprints/Other/S_Item` (`self.Item`))) 0)
    (if (>= (`.Count_8_4FA908A94D8A3E10DFE8349075F8DC5E` (break `/Game/SurvivalGameKit/Blueprints/Other/S_Item` (`self.Item`))) (`local.Harvested Amount L`))
      (bind _output_get (set `self.Item` (make `/Game/SurvivalGameKit/Blueprints/Other/S_Item` _item (- _count (`local.Harvested Amount L`)))))
      (if (not (> (`.Count_8_4FA908A94D8A3E10DFE8349075F8DC5E` (break `/Game/SurvivalGameKit/Blueprints/Other/S_Item` _output_get)) 0))
        (`self.K2_DestroyActor`))
      (return (make `/Game/SurvivalGameKit/Blueprints/Other/S_ItemInventory` (`KismetStringLibrary.Conv_NameToString` (`.RowName` (break `DataTableRowHandle` (`.Item_7_6DD22829457E65E91275E7AC82D14EEF` (break `/Game/SurvivalGameKit/Blueprints/Other/S_Item` (`self.Item`)))))) (`local.Harvested Amount L`)))
      (else
        (return (make `/Game/SurvivalGameKit/Blueprints/Other/S_ItemInventory` (`KismetStringLibrary.Conv_NameToString` (`.RowName` (break `DataTableRowHandle` _item_2))) _count_2))))))

(fn `UserConstructionScript`)