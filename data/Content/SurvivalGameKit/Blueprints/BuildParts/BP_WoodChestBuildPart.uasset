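; Placeable wood chest build part that gives players access to a storage inventory.
; Interaction opens its storage component, first checking the player against the owners list when ownership is required.
; It swaps static meshes for open and closed states and toggles custom depth while targeted.
; Multicast destruction clears the mesh, shatters an optional destructible mesh, then removes the actor after a delay, or immediately without one.
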(event `/Game/SurvivalGameKit/Blueprints/Other/Interfaces/BP_SurvivalInventoryInterface.Interact`
  (params (`Player Component` :type "/Game/SurvivalGameKit/Blueprints/Components/BP_PlayerInventoryComponent Object Reference"))
  ;[0 1 0.09084] Server events
  ;;[1 1 1] Interact
  (set `self.Interacted Player Inventory` `Player Component`)
  (if (`self.Owner Required Interact`)
    (bind _return_value (`self.Check Owners` (`/Game/SurvivalGameKit/Blueprints/Components/BP_PlayerBuildingComponent.Player Name` (`/Game/SurvivalGameKit/Blueprints/Components/BP_PlayerInventoryComponent.Player Building Component` (`self.Interacted Player Inventory`)))))
    (if _return_value
      (`/Game/SurvivalGameKit/Blueprints/Components/BP_MasterInventoryComponent.Interact` (`self.StorageInventoryComponent`) (`self.Interacted Player Inventory`) :!label _label))
    (else
      (goto _label))))

(event `/Game/SurvivalGameKit/Blueprints/Other/Interfaces/BP_SurvivalInventoryInterface.Open Interact Animation`
  ;[0 1 0.09084] Server events
  ;;[1 1 1] Set open static mesh
  (`StaticMeshComponent.SetStaticMesh` (`self.Wood Chest`) "/Game/SurvivalGameKit/Meshes/StaticMeshes/SM_Fire_Treasure002.SM_Fire_Treasure002"))

(event `/Game/SurvivalGameKit/Blueprints/Other/Interfaces/BP_SurvivalInventoryInterface.Target`
  ;[0 0.5089 1] Client events
  ;;[1 1 1] Player target
  (`PrimitiveComponent.SetRenderCustomDepth` (`self.Wood Chest`) true))

(event `/Game/SurvivalGameKit/Blueprints/Other/Interfaces/BP_SurvivalInventoryInterface.Close Interact Animation`
  ;[0 1 0.09084] Server events
  ;;[1 1 1] Set closed static mesh
  (`StaticMeshComponent.SetStaticMesh` (`self.Wood Chest`) "/Game/SurvivalGameKit/Meshes/StaticMeshes/SM_Fire_Treasure003.SM_Fire_Treasure003"))

(event `/Game/SurvivalGameKit/Blueprints/Other/Interfaces/BP_SurvivalInventoryInterface.Not Target`
  ;[0 0.5089 1] Client events
  ;;[1 1 1] Not a player target
  (`PrimitiveComponent.SetRenderCustomDepth` (`self.Wood Chest`) false))

(event `self.Multicast Destroy`
  (bind (_build_part_info_name _build_part_info_type _build_part_info_description _build_part_info_health _build_part_info_takedamage _build_part_info_rotationenabled _build_part_info_rotationincrements _build_part_info_upgradebuildpart _build_part_info_repairitem _build_part_info_blueprintclass _build_part_info_staticmesh _build_part_info_destructiblemesh) (break `/Game/SurvivalGameKit/Blueprints/Other/S_BuildPartInfo` (`self.Build Part Info`)))
  ;[1 0 0] Multicast events
  ;;[1 1 1] Multicast destroy
  (set `self.Pending Destroy` true)
  (`StaticMeshComponent.SetStaticMesh` (`self.Wood Chest`) null)
  (`/Engine/EditorBlueprintResources/StandardMacros.IsValid` (`.DestructibleMesh_52_4F8797AA4A13A416AB00A38BF749C987` (break `/Game/SurvivalGameKit/Blueprints/Other/S_BuildPartInfo` (`self.Build Part Info`)))
    (:`Is Valid`
      (`DestructibleComponent.SetDestructibleMesh` (`self.Destructible`) _build_part_info_destructiblemesh)
      (`DestructibleComponent.ApplyDamage` (`self.DestructibleNoCollision`) 100.0 (`self.K2_GetActorLocation`) (0.0 1.0 0.0) 2.0)
      (`DestructibleComponent.ApplyDamage` (`self.Destructible`) 100.0 (`self.K2_GetActorLocation`) (0.0 1.0 0.0) 2.0)
      (`KismetSystemLibrary.Delay` 5.0)
      (`self.K2_DestroyActor`))
    (:`Is Not Valid`
      (`self.K2_DestroyActor`))))

(fn `UserConstructionScript`)